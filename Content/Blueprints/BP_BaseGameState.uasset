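; Base game state Blueprint that provides a helper for finding which team is ahead on score.
; GetLeadingTeam scans a score array for the highest value and returns it with the matching E_Team value.
; The array index is offset by one when converted to the enum, and ties go to the earliest entry.
; The event graph and construction script contain no logic.
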(fn `GetLeadingTeam`
  (params (Scores :type "Array of Integer"))
  (returns (Team :type "/Game/Data/E_Team Enum") (BiggestScore :type Integer))
  (locals (TEMP_Biggest :type Integer) (TEMP_Index :type Integer))
  (set `local.TEMP_Biggest` (`|GetArrayItem` Scores))
  (set `local.TEMP_Index` 0)
  (for _index (range 1 (`KismetArrayLibrary.Array_Length` Scores))
    (bind _output (`|GetArrayItem` (`local.Scores`) _index))
    (if (> _output (`local.TEMP_Biggest`))
      (set `local.TEMP_Biggest` _output)
      (set `local.TEMP_Index` _index)))
  (return (cast `/Game/Data/E_Team` (`KismetMathLibrary.Conv_IntToByte` (+ (`local.TEMP_Index`) 1))) (`local.TEMP_Biggest`)))

(fn `UserConstructionScript`)