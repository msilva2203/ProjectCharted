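; BP_PlayerSpawner is a team-assigned spawn point that creates a BP_BaseCharacter at its transform and has the given player possess it.
; Each spawn marks it unavailable and starts a one-shot WaitTime timer that restores availability, which IsAvailable reports.
; It also exposes entity-style getters, where GetTeam returns its Team and the rest, such as score, kills and locations, return placeholder defaults.
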(event `SetAvailability`
  (params (NewValue :type Boolean))
  (bind _output_get (set `self.Available` NewValue))
  (if (not _output_get)
    (bind _returnvalue (`KismetSystemLibrary.K2_SetTimerDelegate` (delegate `EVENT_OnWaitEnd`) (`self.WaitTime`)))
    (set `self.Timer_Wait` _returnvalue)))

(event `EVENT_OnWaitEnd`
  (`self.SetAvailability` true))

(fn `GetAssists`
  (returns (Assists :type Integer))
  (return 0))

(fn `GetDeaths`
  (returns (Deaths :type Integer))
  (return 0))

(fn `GetEntityName`
  (returns (Name :type Text))
  (return ""))

(fn `GetFocusLocation`
  (returns (Location :type "Vector Structure"))
  (return (0.0 0.0 0.0)))

(fn `GetGamemode`
  (returns (Gamemode :type "/Game/Data/E_Gamemode Enum"))
  (return "NewEnumerator0"))

(fn `GetKills`
  (returns (Kills :type Integer))
  (return 0))

(fn `GetMoneyLocation`
  (returns (Location :type "Vector Structure"))
  (return (0.0 0.0 0.0)))

(fn `GetScore`
  (returns (Score :type Integer))
  (return 0))

(fn `GetSightLocation`
  (returns (Location :type "Vector Structure"))
  (return (0.0 0.0 0.0)))

(fn `GetTeam`
  (returns (Team :type "/Game/Data/E_Team Enum"))
  (return (`self.Team`)))

(fn `IsAvailable`
  (returns (Available :type Boolean))
  (return (`self.Available`)))

(fn `IsCritical`
  (params (`Hit Bone` :type Name))
  (returns (IsCritical :type Boolean))
  (return false))

(fn `SpawnPlayer`
  (params (Player :type "/Game/Blueprints/BP_BasePlayerController Object Reference"))
  (returns (Character :type "/Game/Blueprints/BP_BaseCharacter Object Reference"))
  (bind _returnvalue (`|SpawnActorFromClass` "/Game/Blueprints/BP_BaseCharacter.BP_BaseCharacter_C" (`self.GetTransform`) "AdjustIfPossibleButAlwaysSpawn" "OverrideRootScale" null null))
  (`Controller.Possess` (`local.Player`) _returnvalue)
  (`self.SetAvailability` false)
  (return _returnvalue))

(fn `UserConstructionScript`)