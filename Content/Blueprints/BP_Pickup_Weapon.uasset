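; Weapon pickup actor that gives a character a weapon, or ammo if that weapon is already owned.
; It takes its display name from the weapon enum and stores the weapon's state and tier.
; On server pickup it either adds the stored reserve ammo to the owned equipment or grants the weapon with its state, then runs the parent pickup logic.
; Interaction is blocked when the player's owned copy is already full.
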(event `self.ReceiveBeginPlay`
  (`parent.ReceiveBeginPlay`)
  (`self.SetPickupName` (`KismetTextLibrary.Conv_StringToText` (`|GetEnumeratorNameAsString` (`self.Weapon`)))))

(event `self.PickupItem (OnServer)`
  (params (Player :type "/Game/Blueprints/BP_BasePlayerController Object Reference") (Character :type "/Game/Blueprints/BP_BaseCharacter Object Reference"))
  (`self.PickupWeapon` Player Character)
  (`parent.PickupItem (OnServer)` Player Character))

(fn `GetWeapon`
  (returns (Weapon :type "/Game/Data/E_Weapon Enum"))
  (return (`self.Weapon`)))

(fn `GetWeaponTier`
  (returns (`Return Value` :type "/Game/Data/E_WeaponTier Enum"))
  (return (`self.WeaponTier`)))

(fn `IsInteractable`
  (returns (`Return Value` :type Boolean))
  (bind _player (`self.Player`))
  (bind (_return_value _equipment) (`/Game/Blueprints/BP_BaseCharacter.HasWeapon` _player (`self.Weapon`)))
  (if _return_value
    (bind (_weapon _isvalid) (`/Game/Blueprints/BP_BaseCharacter.GetEquipment` _player _equipment))
    (if _isvalid
      (return (and (`parent.IsInteractable`) (not (`/Game/Blueprints/BP_BaseWeapon.IsFull` _weapon))))
      (else
        _)))
  (return (`parent.IsInteractable`)))

(fn `PickupWeapon`
  (params (Player :type "/Game/Blueprints/BP_BasePlayerController Object Reference") (Character :type "/Game/Blueprints/BP_BaseCharacter Object Reference"))
  (bind (_return_value _equipment) (`/Game/Blueprints/BP_BaseCharacter.HasWeapon` Character (`self.GetWeapon`)))
  (if _return_value
    (`/Game/Blueprints/BP_BaseCharacter.SERVER_AddAmmo` Character _equipment (`.CurrentReserves_5_E546978B44BA593CEFEF608B8F17996A` (break `/Game/Data/F_WeaponState` (`self.WeaponState`))))
    (else
      (`/Game/Blueprints/BP_BaseCharacter.SERVER_PickupWeapon` Character (`self.Weapon`) (`self.WeaponState`) false true))))

(fn `SetWeaponState`
  (params (NewState :type "/Game/Data/F_WeaponState Structure"))
  (set `self.WeaponState` NewState))

(fn `SetWeaponTier`
  (params (WeaponTier :type "/Game/Data/E_WeaponTier Enum" :default "NewEnumerator0"))
  (set `self.WeaponTier` WeaponTier))

(fn `UserConstructionScript`)