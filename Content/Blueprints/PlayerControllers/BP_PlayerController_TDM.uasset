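; Player controller for Team Deathmatch that creates and controls the TDM HUD, game feed, scoreboard and match results.
; Each kill adds a point to the player's team score on the TDM game state.
; Scoreboard updates split player states into own team and enemies, then sort each with a nested-loop IsWorse swap.
; ShowResults compares the winning team to the player's to pick the outcome shown on the scoreboard and passed to OnGameResult.
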(event `self.ReceiveBeginPlay`
  (`parent.ReceiveBeginPlay`)
  (bind _asbp_game_state_tdm (cast `/Game/Blueprints/Gamestates/BP_GameState_TDM` (`GameplayStatics.GetGameState`)))
  (set `self.GameState_TDM` _asbp_game_state_tdm))

(event `/Game/BlueprintInterfaces/BI_Game.AddKill`
  (`parent.AddKill`)
  (bind _team (`/Game/BlueprintInterfaces/BI_Game.GetTeam`))
  (`/Game/Blueprints/Gamestates/BP_GameState_TDM.OffsetTeamScore` (`self.GameState_TDM`) _team 1))

(fn `AddToGameFeed`
  (params (`Feed Data` :type "/Game/Data/F_FeedData Structure"))
  (`/Game/UserInterface/Gameplay/Components/WBP_FeedBox.AddToGameFeed` (`/Game/UserInterface/Gameplay/WBP_GameHUD_TDM.WBP_FeedBox` (`self.GameHUD_TDM`)) `Feed Data`))

(fn `CreateGameHUD`
  (bind _returnvalue (`|CreateWidget` "/Game/UserInterface/Gameplay/WBP_GameHUD_TDM.WBP_GameHUD_TDM_C" (`GameplayStatics.GetPlayerController` 0)))
  (bind _output_get (set `self.GameHUD_TDM` _returnvalue))
  (`UserWidget.AddToViewport` _output_get 0)
  (`self.HideGameHUD`))

(fn `GetGameHUD`
  (returns (Widget :type "UserWidget Object Reference"))
  (return (`self.GameHUD_TDM`)))

(fn `GetGameHUD_0`
  (returns (`Return Value` :type "/Game/UserInterface/Gameplay/WBP_GameHUD_TDM Object Reference"))
  (return (`self.GameHUD_TDM`)))

(fn `HideGameHUD`
  (`Widget.SetVisibility` (`self.GameHUD_TDM`) "Collapsed"))

(fn `HideScoreboard`
  (`parent.HideScoreboard`)
  (`/Game/UserInterface/Gameplay/WBP_GameHUD_TDM.HideScoreboard` (`self.GameHUD_TDM`)))

(fn `ShowGameHUD`
  (`Widget.SetVisibility` (`self.GameHUD_TDM`) "Visible"))

(fn `ShowResults`
  (params (WinningTeam :type "/Game/Data/E_Team Enum" :default "NewEnumerator0"))
  (`parent.ShowResults` WinningTeam)
  (bind _team (`/Game/BlueprintInterfaces/BI_Game.GetTeam`))
  (if (`|EnumEquality` _team WinningTeam)
    (`/Game/UserInterface/Gameplay/Scoreboards/WBP_Scoreboard_TDM.ShowResult` (`/Game/UserInterface/Gameplay/WBP_GameHUD_TDM.WBP_Scoreboard_TDM` (`self.GameHUD_TDM`)) "NewEnumerator1")
    (`self.OnGameResult` "NewEnumerator1")
    (elif (`|EnumEquality` WinningTeam "NewEnumerator0")
      (`/Game/UserInterface/Gameplay/Scoreboards/WBP_Scoreboard_TDM.ShowResult` (`/Game/UserInterface/Gameplay/WBP_GameHUD_TDM.WBP_Scoreboard_TDM` (`self.GameHUD_TDM`)) "NewEnumerator3")
      (`self.OnGameResult` "NewEnumerator3")
      (else
        (`/Game/UserInterface/Gameplay/Scoreboards/WBP_Scoreboard_TDM.ShowResult` (`/Game/UserInterface/Gameplay/WBP_GameHUD_TDM.WBP_Scoreboard_TDM` (`self.GameHUD_TDM`)) "NewEnumerator2")
        (`self.OnGameResult` "NewEnumerator2")))))

(fn `ShowScoreboard`
  (`parent.ShowScoreboard`)
  (`/Game/UserInterface/Gameplay/WBP_GameHUD_TDM.ShowScoreboard` (`self.GameHUD_TDM`)))

(fn `Update Scoreboard`
  (locals (TEMP_Team :type "Array of /Game/Blueprints/PlayerStates/BP_PlayerState_TDM Object Reference") (TEMP_Enemies :type "Array of /Game/Blueprints/PlayerStates/BP_PlayerState_TDM Object Reference") (TEMP_1 :type "/Game/Blueprints/PlayerStates/BP_PlayerState_TDM Object Reference") (TEMP_2 :type "/Game/Blueprints/PlayerStates/BP_PlayerState_TDM Object Reference"))
  (bind _returnvalue (- (`KismetArrayLibrary.Array_Length` (`local.TEMP_Enemies`)) 1))
  (bind _returnvalue_2 (- (`KismetArrayLibrary.Array_Length` (`local.TEMP_Team`)) 1))
  (for _array_element (`self.PlayerStates`)
    (bind _team (`/Game/BlueprintInterfaces/BI_Game.GetTeam` _array_element))
    (bind _team_2 (`/Game/BlueprintInterfaces/BI_Game.GetTeam`))
    (if (`|EnumEquality` _team_2 _team)
      (bind _asbp_player_state_tdm (cast `/Game/Blueprints/PlayerStates/BP_PlayerState_TDM` _array_element :!pure true))
      (`KismetArrayLibrary.Array_Add` (`local.TEMP_Team`) _asbp_player_state_tdm)
      (else
        (`KismetArrayLibrary.Array_Add` (`local.TEMP_Enemies`) _asbp_player_state_tdm))))
  (for _index (range (+ _returnvalue_2 1))
    (for _index_2 (range _index (+ _returnvalue_2 1))
      (bind _output (`|GetArrayItem` (`local.TEMP_Team`) _index))
      (bind _output_2 (`|GetArrayItem` (`local.TEMP_Team`) _index_2))
      (if (`/Game/Blueprints/PlayerStates/BP_PlayerState_TDM.Is Worse` _output _output_2)
        (bind _output_get (set `local.TEMP_1` _output))
        (bind _output_get_2 (set `local.TEMP_2` _output_2))
        (`KismetArrayLibrary.Array_Set` (`local.TEMP_Team`) _index _output_get_2)
        (`KismetArrayLibrary.Array_Set` (`local.TEMP_Team`) _index_2 _output_get))))
  (for _index_3 (range (+ _returnvalue 1))
    (for _index_4 (range _index_3 (+ _returnvalue 1))
      (bind _output_3 (`|GetArrayItem` (`local.TEMP_Enemies`) _index_3))
      (bind _output_4 (`|GetArrayItem` (`local.TEMP_Enemies`) _index_4))
      (if (`/Game/Blueprints/PlayerStates/BP_PlayerState_TDM.Is Worse` _output_3 _output_4)
        (bind _output_get_3 (set `local.TEMP_1` _output_3))
        (bind _output_get_4 (set `local.TEMP_2` _output_4))
        (`KismetArrayLibrary.Array_Set` (`local.TEMP_Enemies`) _index_3 _output_get_4)
        (`KismetArrayLibrary.Array_Set` (`local.TEMP_Enemies`) _index_4 _output_get_3))))
  (`/Game/UserInterface/Gameplay/Scoreboards/WBP_Scoreboard_TDM.UpdateScoreboard` (`/Game/UserInterface/Gameplay/WBP_GameHUD_TDM.WBP_Scoreboard_TDM` (`self.GameHUD_TDM`)) (`local.TEMP_Team`) (`local.TEMP_Enemies`)))

(fn `UserConstructionScript`
  (`parent.UserConstructionScript`))