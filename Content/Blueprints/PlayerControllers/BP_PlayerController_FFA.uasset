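; Player controller for the free-for-all game mode, extending a parent controller with FFA scoring and HUD handling.
; On BeginPlay it caches the FFA game state, and each kill adds a point to the player's team score there.
; It creates the game HUD from the team deathmatch widget class, starts it collapsed, and provides show, hide and getter functions.
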(event `self.ReceiveBeginPlay`
  (`parent.ReceiveBeginPlay`)
  (bind _asbp_game_state_ffa (cast `/Game/Blueprints/Gamestates/BP_GameState_FFA` (`GameplayStatics.GetGameState`)))
  (set `self.GameState_FFA` _asbp_game_state_ffa))

(event `/Game/BlueprintInterfaces/BI_Game.AddKill`
  (`parent.AddKill`)
  (bind _team (`/Game/BlueprintInterfaces/BI_Game.GetTeam`))
  (`/Game/Blueprints/Gamestates/BP_GameState_FFA.OffsetTeamScore` (`self.GameState_FFA`) _team 1))

(fn `CreateGameHUD`
  (bind _returnvalue (`|CreateWidget` "/Game/UserInterface/Gameplay/WBP_GameHUD_TDM.WBP_GameHUD_TDM_C" (`GameplayStatics.GetPlayerController` 0)))
  (bind _output_get (set `self.GameHUD_FFA` _returnvalue))
  (`UserWidget.AddToViewport` _output_get 0)
  (`self.HideGameHUD`))

(fn `GetGameHUD`
  (returns (GameHUD_FFA :type "/Game/UserInterface/Gameplay/WBP_GameHUD_TDM Object Reference"))
  (return (`self.GameHUD_FFA`)))

(fn `HideGameHUD`
  (`Widget.SetVisibility` (`self.GameHUD_FFA`) "Collapsed"))

(fn `ShowGameHUD`
  (`Widget.SetVisibility` (`self.GameHUD_FFA`) "SelfHitTestInvisible"))

(fn `UserConstructionScript`
  (`parent.UserConstructionScript`))