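; Death camera actor that becomes the first player's view and turns toward the killer.
; ActivateCamera stores the killer, places the actor and switches the view target; DeactivateCamera only stops the tracking.
; While open, Tick aims the camera at the killer's focus location, interpolating each frame from the actor's rotation rather than the camera's.
; A distance-based FOV zoom, narrower for farther killers, exists but never runs.
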(event `self.ReceiveTick`
  (params (DeltaSeconds :type "Float (single-precision)"))
  (if (`self.Open`)
    (`/Engine/EditorBlueprintResources/StandardMacros.IsValid` (`self.Killer`)
      (:`Is Valid`
        (`self.UpdateCameraRotation`)))))

(fn `ActivateCamera`
  (params (Killer :type "Actor Object Reference") (Location :type "Vector Structure") (Rotation :type "Rotator Structure"))
  (set `self.Killer` Killer)
  (set `self.Open` true)
  (`self.K2_SetActorLocation` (`local.Location`))
  (`self.K2_SetActorRotation` (`local.Rotation`))
  (`PlayerController.SetViewTargetWithBlend` (`GameplayStatics.GetPlayerController` 0) self 0.0 "VTBlend_Linear" 0.0 false))

(fn `DeactivateCamera`
  (set `self.Open` false))

(fn `UpdateCameraFOV`
  (bind _location (message `/Game/BlueprintInterfaces/BI_Game.GetFocusLocation` (`self.Killer`)))
  (`CameraComponent.SetFieldOfView` (`self.Camera`) (`KismetMathLibrary.FInterpTo` (`CameraComponent.FieldOfView` (`self.Camera`)) (+ (* (- 1.0 (/ (- (`KismetMathLibrary.FClamp` (`KismetMathLibrary.Vector_Distance` _location (`self.K2_GetActorLocation`)) 100.0 2000.0) 100.0) 1900.0)) 60.0) 40.0) (`GameplayStatics.GetWorldDeltaSeconds`) 10.0)))

(fn `UpdateCameraRotation`
  (bind _location (message `/Game/BlueprintInterfaces/BI_Game.GetFocusLocation` (`self.Killer`)))
  (`SceneComponent.K2_SetWorldRotation` (`self.Camera`) (`KismetMathLibrary.RInterpTo` (`self.K2_GetActorRotation`) (`KismetMathLibrary.FindLookAtRotation` (`self.K2_GetActorLocation`) _location) (`GameplayStatics.GetWorldDeltaSeconds`) (`self.Speed_Rotation`)) false false))

(fn `UserConstructionScript`)