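; Game state for the TTDM mode that holds replicated scores for three teams, the score goal and the match time.
; Setter, getter and offset functions manage the values, with team scores selected by team enum and only TEAM1 to TEAM3 stored.
; RepNotify handlers push each change to the TTDM HUD through a lazily cached local player controller.
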(fn `GetPlayerController`
  (returns (PlayerController :type "/Game/Blueprints/PlayerControllers/BP_PlayerController_TTDM Object Reference"))
  (`/Engine/EditorBlueprintResources/StandardMacros.IsValid` (`self.PlayerController`)
    (:`Is Valid`
      (return (`self.PlayerController`)))
    (:`Is Not Valid`
      (bind _asbp_player_controller_ttdm (cast `/Game/Blueprints/PlayerControllers/BP_PlayerController_TTDM` (`GameplayStatics.GetPlayerController` 0))
        (:`then`
          (bind _output_get (set `self.PlayerController` _asbp_player_controller_ttdm))
          (return _output_get))
        (:`CastFailed`
          (return (`self.PlayerController`)))))))

(fn `GetTeamScore`
  (params (Team :type "/Game/Data/E_Team Enum" :default "NewEnumerator0"))
  (returns (Score :type Integer))
  (return (select `/Game/Data/E_Team` (`local.Team`) :`NewEnumerator1` (`self.Score_Team1`) :`NewEnumerator2` (`self.Score_Team2`) :`NewEnumerator3` (`self.Score_Team3`))))

(fn `OffsetTeamScore`
  (params (Team :type "/Game/Data/E_Team Enum" :default "NewEnumerator0") (Offset :type Integer))
  (`self.SetTeamScore` Team (+ Offset (`self.GetTeamScore` Team))))

(fn `OnRep_Score_Goal`
  (`/Game/UserInterface/Gameplay/WBP_GameHUD_TTDM.SetGoal` (`/Game/Blueprints/PlayerControllers/BP_PlayerController_TTDM.GameHUD_TTDM` (`self.GetPlayerController`)) (`self.Score_Goal`)))

(fn `OnRep_Score_Team1`
  (`/Game/UserInterface/Gameplay/WBP_GameHUD_TTDM.UpdateTeamScore` (`/Game/Blueprints/PlayerControllers/BP_PlayerController_TTDM.GameHUD_TTDM` (`self.GetPlayerController`)) "NewEnumerator1" (`self.Score_Team1`)))

(fn `OnRep_Score_Team2`
  (`/Game/UserInterface/Gameplay/WBP_GameHUD_TTDM.UpdateTeamScore` (`/Game/Blueprints/PlayerControllers/BP_PlayerController_TTDM.GameHUD_TTDM` (`self.GetPlayerController`)) "NewEnumerator2" (`self.Score_Team2`)))

(fn `OnRep_Score_Team3`
  (`/Game/UserInterface/Gameplay/WBP_GameHUD_TTDM.UpdateTeamScore` (`/Game/Blueprints/PlayerControllers/BP_PlayerController_TTDM.GameHUD_TTDM` (`self.GetPlayerController`)) "NewEnumerator3" (`self.Score_Team3`)))

(fn `OnRep_Time`
  (`/Game/UserInterface/Gameplay/WBP_GameHUD_TTDM.SetTime` (`/Game/Blueprints/PlayerControllers/BP_PlayerController_TTDM.GameHUD_TTDM` (`self.GetPlayerController`)) (`self.Time`)))

(fn `SetGoal`
  (params (NewGoal :type Integer))
  (set `self.Score_Goal` NewGoal))

(fn `SetTeamScore`
  (params (Team :type "/Game/Data/E_Team Enum" :default "NewEnumerator0") (Score :type Integer))
  (switch `/Game/Data/E_Team` Team
    (:`NewEnumerator1`
      (set `self.Score_Team1` (`local.Score`)))
    (:`NewEnumerator2`
      (set `self.Score_Team2` (`local.Score`)))
    (:`NewEnumerator3`
      (set `self.Score_Team3` (`local.Score`)))))

(fn `SetTime`
  (params (NewTime :type Integer))
  (set `self.Time` NewTime))

(fn `UserConstructionScript`)