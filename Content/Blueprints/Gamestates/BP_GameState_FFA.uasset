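; Game state for free-for-all matches, tracking the timer, score goal and separate scores for eight team slots.
; Score changes through SetTeamScore or OffsetTeamScore check against the goal, and reaching it sets the winning team and ends the match through the game mode.
; RepNotifies push time, goal and scores to the local HUD via a cached player controller, showing the player's score against the best rival score.
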(fn `CheckForWin`
  (params (Team :type "/Game/Data/E_Team Enum" :default "NewEnumerator0") (Score :type Integer))
  (bind _base_gamemode (`/Game/BlueprintLibraries/Game.GetBaseGamemode`))
  (if (>= Score (`self.Goal`))
    (`/Game/Blueprints/BP_BaseGamemode.SetWinningTeam` _base_gamemode (`local.Team`))
    (`/Game/Blueprints/BP_BaseGamemode.EndMatch` _base_gamemode true)))

(fn `GetBiggestScore`
  (params (TeamToIgnore :type "/Game/Data/E_Team Enum" :default "NewEnumerator0"))
  (returns (ReturnValue :type Integer))
  (locals (TEMP_Array :type "Array of Integer") (TEMP_Biggest :type Integer))
  (bind _output_get (set `local.TEMP_Array` (`|MakeArray` (`self.Score_Team1`) (`self.Score_Team2`) (`self.Score_Team3`) (`self.Score_Team4`) (`self.Score_Team5`) (`self.Score_Team6`) (`self.Score_Team7`) (`self.Score_Team8`))))
  (for (_array_element _array_index) _output_get
    (if (`|EnumInequality` (`local.TeamToIgnore`) (cast `/Game/Data/E_Team` (`KismetMathLibrary.Conv_IntToByte` (+ _array_index 1))))
      (if (>= _array_element (`local.TEMP_Biggest`))
        (set `local.TEMP_Biggest` _array_element))))
  (return (`local.TEMP_Biggest`)))

(fn `GetPlayerController`
  (returns (PlayerController :type "/Game/Blueprints/PlayerControllers/BP_PlayerController_FFA Object Reference"))
  (`/Engine/EditorBlueprintResources/StandardMacros.IsValid` (`self.PlayerController`)
    (:`Is Valid`
      (return (`self.PlayerController`)))
    (:`Is Not Valid`
      (bind _asbp_player_controller_ffa (cast `/Game/Blueprints/PlayerControllers/BP_PlayerController_FFA` (`GameplayStatics.GetPlayerController` 0)))
      (bind _output_get (set `self.PlayerController` _asbp_player_controller_ffa))
      (return _output_get))))

(fn `GetTeamScore`
  (params (Team :type "/Game/Data/E_Team Enum" :default "NewEnumerator0"))
  (returns (Score :type Integer))
  (return (select `/Game/Data/E_Team` (`local.Team`) :`NewEnumerator1` (`self.Score_Team1`) :`NewEnumerator2` (`self.Score_Team2`) :`NewEnumerator3` (`self.Score_Team3`) :`NewEnumerator4` (`self.Score_Team4`) :`NewEnumerator5` (`self.Score_Team5`) :`NewEnumerator6` (`self.Score_Team6`) :`NewEnumerator7` (`self.Score_Team7`) :`NewEnumerator8` (`self.Score_Team8`))))

(fn `OffsetTeamScore`
  (params (Team :type "/Game/Data/E_Team Enum" :default "NewEnumerator0") (Offset :type Integer))
  (switch `/Game/Data/E_Team` Team
    (:`NewEnumerator1`
      (`self.SetTeamScore` "NewEnumerator1" (+ (`self.Score_Team1`) (`local.Offset`))))
    (:`NewEnumerator2`
      (`self.SetTeamScore` "NewEnumerator2" (+ (`self.Score_Team2`) (`local.Offset`))))
    (:`NewEnumerator3`
      (`self.SetTeamScore` "NewEnumerator3" (+ (`self.Score_Team3`) (`local.Offset`))))
    (:`NewEnumerator4`
      (`self.SetTeamScore` "NewEnumerator4" (+ (`self.Score_Team4`) (`local.Offset`))))
    (:`NewEnumerator5`
      (`self.SetTeamScore` "NewEnumerator5" (+ (`self.Score_Team5`) (`local.Offset`))))
    (:`NewEnumerator6`
      (`self.SetTeamScore` "NewEnumerator6" (+ (`self.Score_Team6`) (`local.Offset`))))
    (:`NewEnumerator7`
      (`self.SetTeamScore` "NewEnumerator7" (+ (`self.Score_Team7`) (`local.Offset`))))
    (:`NewEnumerator8`
      (`self.SetTeamScore` "NewEnumerator8" (+ (`self.Score_Team8`) (`local.Offset`))))))

(fn `OnRep_Goal`
  (`/Game/UserInterface/Gameplay/WBP_GameHUD_FFA.SetGoal` (`/Game/Blueprints/PlayerControllers/BP_PlayerController_FFA.GetGameHUD_0` (`self.GetPlayerController`)) (`self.Goal`)))

(fn `OnRep_Score_Team1`
  (`self.UpdateScoreHUD`))

(fn `OnRep_Score_Team2`
  (`self.UpdateScoreHUD`))

(fn `OnRep_Score_Team3`
  (`self.UpdateScoreHUD`))

(fn `OnRep_Score_Team4`
  (`self.UpdateScoreHUD`))

(fn `OnRep_Score_Team5`
  (`self.UpdateScoreHUD`))

(fn `OnRep_Score_Team6`
  (`self.UpdateScoreHUD`))

(fn `OnRep_Score_Team7`
  (`self.UpdateScoreHUD`))

(fn `OnRep_Score_Team8`
  (`self.UpdateScoreHUD`))

(fn `OnRep_Time`
  (`/Game/UserInterface/Gameplay/WBP_GameHUD_FFA.SetTime` (`/Game/Blueprints/PlayerControllers/BP_PlayerController_FFA.GetGameHUD_0` (`self.GetPlayerController`)) (`self.Time`)))

(fn `SetGoal`
  (params (NewValue :type Integer))
  (set `self.Goal` NewValue))

(fn `SetTeamScore`
  (params (Team :type "/Game/Data/E_Team Enum" :default "NewEnumerator0") (Score :type Integer))
  (bind _score (`local.Score`))
  (switch `/Game/Data/E_Team` Team
    (:`NewEnumerator1`
      (bind _output_get (set `self.Score_Team1` _score))
      (`self.CheckForWin` "NewEnumerator1" _output_get))
    (:`NewEnumerator2`
      (bind _output_get_2 (set `self.Score_Team2` _score))
      (`self.CheckForWin` "NewEnumerator2" _output_get_2))
    (:`NewEnumerator3`
      (bind _output_get_3 (set `self.Score_Team3` _score))
      (`self.CheckForWin` "NewEnumerator3" _output_get_3))
    (:`NewEnumerator4`
      (bind _output_get_4 (set `self.Score_Team4` _score))
      (`self.CheckForWin` "NewEnumerator4" _output_get_4))
    (:`NewEnumerator5`
      (bind _output_get_5 (set `self.Score_Team5` _score))
      (`self.CheckForWin` "NewEnumerator5" _output_get_5))
    (:`NewEnumerator6`
      (bind _output_get_6 (set `self.Score_Team6` _score))
      (`self.CheckForWin` "NewEnumerator6" _output_get_6))
    (:`NewEnumerator7`
      (bind _output_get_7 (set `self.Score_Team7` _score))
      (`self.CheckForWin` "NewEnumerator7" _output_get_7))
    (:`NewEnumerator8`
      (bind _output_get_8 (set `self.Score_Team8` _score))
      (`self.CheckForWin` "NewEnumerator8" _output_get_8))))

(fn `SetTime`
  (params (NewValue :type Integer))
  (set `self.Time` NewValue))

(fn `UpdateScoreHUD`
  (bind _team (message `/Game/BlueprintInterfaces/BI_Game.GetTeam` (`GameplayStatics.GetPlayerController` 0)))
  (bind _returnvalue (`self.GetBiggestScore` _team))
  (`/Game/UserInterface/Gameplay/WBP_GameHUD_FFA.UpdateScores` (`/Game/Blueprints/PlayerControllers/BP_PlayerController_FFA.GetGameHUD_0` (`self.GetPlayerController`)) (`self.GetTeamScore` _team) _returnvalue))

(fn `UserConstructionScript`)