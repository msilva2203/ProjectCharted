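; Team Deathmatch game state that holds both teams' scores, the score goal and the match time.
; Simple functions set these values or offset a team's score, and RepNotify handlers push each change to the local player's game HUD.
; The handlers reach the HUD through a lazily cached TDM player controller, cast from player index 0.
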(fn `GetPlayerController`
  (returns (PlayerController :type "/Game/Blueprints/PlayerControllers/BP_PlayerController_TDM Object Reference"))
  (`/Engine/EditorBlueprintResources/StandardMacros.IsValid` (`self.PlayerController`)
    (:`Is Valid`
      (return (`self.PlayerController`)))
    (:`Is Not Valid`
      (bind _asbp_player_controller_tdm (cast `/Game/Blueprints/PlayerControllers/BP_PlayerController_TDM` (`GameplayStatics.GetPlayerController` 0))
        (:`then`
          (set `self.PlayerController` _asbp_player_controller_tdm)
          (return (`self.PlayerController`)))
        (:`CastFailed`
          (return (`self.PlayerController`)))))))

(fn `OffsetTeamScore`
  (params (Team :type "/Game/Data/E_Team Enum" :default "NewEnumerator0") (Offset :type Integer))
  (switch `/Game/Data/E_Team` Team
    (:`NewEnumerator1`
      (set `self.Score_Team1` (+ Offset (`self.Score_Team1`))))
    (:`NewEnumerator2`
      (set `self.Score_Team2` (+ Offset (`self.Score_Team2`))))))

(fn `OnRep_Score_Goal`
  (`/Game/UserInterface/Gameplay/WBP_GameHUD_TDM.SetGoal` (`/Game/Blueprints/PlayerControllers/BP_PlayerController_TDM.GetGameHUD` (`self.GetPlayerController`)) (`self.Score_Goal`)))

(fn `OnRep_Score_Team1`
  (`/Game/UserInterface/Gameplay/WBP_GameHUD_TDM.UpdateTeamScore` (`/Game/Blueprints/PlayerControllers/BP_PlayerController_TDM.GetGameHUD` (`self.GetPlayerController`)) "NewEnumerator1" (`self.Score_Team1`)))

(fn `OnRep_Score_Team2`
  (`/Game/UserInterface/Gameplay/WBP_GameHUD_TDM.UpdateTeamScore` (`/Game/Blueprints/PlayerControllers/BP_PlayerController_TDM.GetGameHUD` (`self.GetPlayerController`)) "NewEnumerator2" (`self.Score_Team2`)))

(fn `OnRep_Time`
  (`/Game/UserInterface/Gameplay/WBP_GameHUD_TDM.SetTime` (`/Game/Blueprints/PlayerControllers/BP_PlayerController_TDM.GetGameHUD` (`self.GetPlayerController`)) (`self.Time`)))

(fn `SetGoal`
  (params (NewValue :type Integer))
  (set `self.Score_Goal` NewValue))

(fn `SetTeamScore`
  (params (Team :type "/Game/Data/E_Team Enum" :default "NewEnumerator0") (Score :type Integer))
  (bind _score (`local.Score`))
  (switch `/Game/Data/E_Team` Team
    (:`NewEnumerator1`
      (set `self.Score_Team1` _score))
    (:`NewEnumerator2`
      (set `self.Score_Team2` _score))))

(fn `SetTime`
  (params (NewValue :type Integer))
  (set `self.Time` NewValue))

(fn `UserConstructionScript`)