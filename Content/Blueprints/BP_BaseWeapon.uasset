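; Base hitscan weapon that reads its stats from WeaponData and handles firing, reloading and equipping for its owning player.
; Input drives a looping timer for automatic fire, with a delayed lock enforcing shot spacing.
; Camera traces send damage through the player's server RPC to BI_Game actors.
; Ammo changes locally and syncs to the server on trigger release or reload, with reserves including loaded rounds; burst getters are unused here.
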(event `Activate`
  (if (and (not (`self.IsMagEmpty`)) (not (`self.Locked`)))
    (`self.Shoot`)
    (if (and (`self.IsFullAuto`) (not (`self.IsMagEmpty`)))
      (bind _returnvalue (`KismetSystemLibrary.K2_SetTimerDelegate` (`|CreateDelegate` :!event `Shoot`) (`self.GetShotInterval`) true))
      (set `self.Timer_Shooting` _returnvalue)
      (else
        (`self.Deactivate`)))))

(event `Deactivate`
  (`self.SERVER_SetState` (`self.WeaponState`))
  (`KismetSystemLibrary.K2_ClearAndInvalidateTimerHandle` (`self.Timer_Shooting`))
  (if (and (not (`self.Locked`)) (`self.Shooting`))
    (set `self.Locked` true)
    (`KismetSystemLibrary.Delay` (`self.GetShotInterval`))
    (set `self.Locked` false)
    (set `self.Shooting` false)
    (if (and (`self.Holding`) (`self.IsFullAuto`))
      (`self.Activate`))))

(event `Shoot`
  (`self.WeaponAttack`)
  (set `self.Shooting` true)
  (`self.OffsetMag` -1)
  (`self.OffsetReserves` -1)
  (`/Game/Blueprints/BP_BasePlayerController.UpdateCurrentWeaponState` (`self.OwnerPlayer`) (`self.WeaponState`))
  (if (`self.IsMagEmpty`)
    (`self.Deactivate`)))

(event `SERVER_SetState`
  (params (WeaponState :type "/Game/Data/F_WeaponState Structure"))
  (bind _output_get (set `self.WeaponState` WeaponState))
  (`self.CLIENT_SetState` _output_get))

(event `CLIENT_SetState`
  (params (WeaponState :type "/Game/Data/F_WeaponState Structure"))
  (set `self.WeaponState` WeaponState)
  (if (`self.IsEquipped`)
    (`/Game/Blueprints/BP_BasePlayerController.UpdateCurrentWeaponState` (`self.OwnerPlayer`) (`self.WeaponState`))))

(event `InputAction|Shoot`
  (params (Key :type "Key Structure"))
  (:`Pressed`
    (set `self.Holding` true)
    (`self.Activate`))
  (:`Released`
    (set `self.Holding` false)
    (`self.Deactivate`)))

(event `InputAction|Reload`
  (params (Key :type "Key Structure"))
  (:`Pressed`
    (`self.OffsetMag` (- (`self.GetCurrentReserves`) (`self.Get Current Mag Ammo`)))
    (`self.SERVER_SetState` (`self.WeaponState`))))

(fn `Equip`
  (params (IsLocal :type Boolean))
  (bind _ownerplayer (`self.OwnerPlayer`))
  (set `self.Local` IsLocal)
  (set `self.Equipped` true)
  (if (`local.IsLocal`)
    (`self.EnableInput` (`GameplayStatics.GetPlayerController` 0))
    (`/Game/Blueprints/BP_BasePlayerController.SetNewWeapon` _ownerplayer (`self.GetMagSize`))
    (`/Game/Blueprints/BP_BasePlayerController.UpdateCurrentWeaponState` _ownerplayer (`self.WeaponState`))))

(fn `Get Current Mag Ammo`
  (returns (CurrentMag :type Integer))
  (return (`.CurrentMag_4_8FD752C1476216EC4CC2E1AD0AB66662` (break `/Game/Data/F_WeaponState` (`self.WeaponState`)))))

(fn `GetBurstTimes`
  (returns (BurstTimes :type Integer))
  (return (`.BurstTimes_21_09949BCB4DD583CED97EBDBE1BFAE635` (break `/Game/Data/F_Weapon` (`self.WeaponData`)))))

(fn `GetCriticalDamage`
  (returns (ReturnValue :type "Float (double-precision)"))
  (bind (_name _weapon _equipment _tier _damage _criticalmultiplier) (break `/Game/Data/F_Weapon` (`self.WeaponData`)))
  (return (* _damage _criticalmultiplier)))

(fn `GetCurrentReserves`
  (returns (CurrentReserves :type Integer))
  (return (`.CurrentReserves_5_E546978B44BA593CEFEF608B8F17996A` (break `/Game/Data/F_WeaponState` (`self.WeaponState`)))))

(fn `GetDamage`
  (returns (Damage :type "Float (double-precision)"))
  (return (`.Damage_30_DF4AE89E49618FDD61035C86D4ADB3C6` (break `/Game/Data/F_Weapon` (`self.WeaponData`)))))

(fn `GetEquipment`
  (returns (Equipment :type "/Game/Data/E_Equipment Enum"))
  (return (`.Equipment_35_C9BB2FB943021327A829BA989B650171` (break `/Game/Data/F_Weapon` (`self.WeaponData`)))))

(fn `GetMagSize`
  (returns (MagSize :type Integer))
  (return (`.MagSize_9_34ACCDEB4D1ECB0A357E81B7846EF234` (break `/Game/Data/F_Weapon` (`self.WeaponData`)))))

(fn `GetMaxReserves`
  (returns (MaxReserves :type Integer))
  (return (`.MaxReserves_12_47E8AF19456C23FB659A86BD9A7F19D6` (break `/Game/Data/F_Weapon` (`self.WeaponData`)))))

(fn `GetRange`
  (returns (Range :type "Float (double-precision)"))
  (return (`.Range_27_5388CA5A4EB0649F4D62F3869F90FA31` (break `/Game/Data/F_Weapon` (`self.WeaponData`)))))

(fn `GetShotInterval`
  (returns (ShotInterval :type "Float (double-precision)"))
  (return (`.ShotInterval_24_D6D9CC57478FA29617F4279E29EB567C` (break `/Game/Data/F_Weapon` (`self.WeaponData`)))))

(fn `GetWeaponEnum`
  (returns (Weapon :type "/Game/Data/E_Weapon Enum"))
  (return (`.Weapon_38_5B83CDD84503071435143599DE1CA680` (break `/Game/Data/F_Weapon` (`self.WeaponData`)))))

(fn `GetWeaponName`
  (returns (Name :type Text))
  (return (`.Name_6_EB71841C4C7AC8544E4C0A82C58FCBC2` (break `/Game/Data/F_Weapon` (`self.WeaponData`)))))

(fn `IsBurst`
  (returns (IsBurst :type Boolean))
  (return (`.IsBurst_18_21FF6C044BA0DC0C4CFAAC977BDF4381` (break `/Game/Data/F_Weapon` (`self.WeaponData`)))))

(fn `IsEmpty`
  (returns (ReturnValue :type Boolean))
  (return (<= (`.CurrentReserves_5_E546978B44BA593CEFEF608B8F17996A` (break `/Game/Data/F_WeaponState` (`self.WeaponState`))) 0)))

(fn `IsEquipped`
  (returns (`Return Value` :type Boolean))
  (return (`self.Equipped`)))

(fn `IsFull`
  (returns (ReturnValue :type Boolean))
  (return (>= (`.CurrentReserves_5_E546978B44BA593CEFEF608B8F17996A` (break `/Game/Data/F_WeaponState` (`self.WeaponState`))) (`.MaxReserves_12_47E8AF19456C23FB659A86BD9A7F19D6` (break `/Game/Data/F_Weapon` (`self.WeaponData`))))))

(fn `IsFullAuto`
  (returns (IsAutomatic :type Boolean))
  (return (`.IsAutomatic_16_80C3F7714EF57D7D38E4FAA06EA58A5A` (break `/Game/Data/F_Weapon` (`self.WeaponData`)))))

(fn `IsLocal`
  (returns (Local :type Boolean))
  (return (`self.Local`)))

(fn `IsMagEmpty`
  (returns (ReturnValue :type Boolean))
  (return (<= (`.CurrentMag_4_8FD752C1476216EC4CC2E1AD0AB66662` (break `/Game/Data/F_WeaponState` (`self.WeaponState`))) 0)))

(fn `OffsetMag`
  (params (Offset :type Integer))
  (bind _currentmag (break `/Game/Data/F_WeaponState` (`self.WeaponState`)))
  (`|VariableSetRef` _currentmag (`KismetMathLibrary.Clamp` (+ Offset _currentmag) 0 (`self.GetMagSize`))))

(fn `OffsetReserves`
  (params (Offset :type Integer) (UpdateClient :type Boolean))
  (bind (_currentmag _currentreserves) (break `/Game/Data/F_WeaponState` (`self.WeaponState`)))
  (`|VariableSetRef` _currentreserves (`KismetMathLibrary.Clamp` (+ Offset _currentreserves) 0 (`self.GetMaxReserves`)))
  (if UpdateClient
    (`self.SERVER_SetState` (`self.WeaponState`))))

(fn `OnRep_WeaponState`
  (if (`self.IsEquipped`)
    (if (`self.IsLocal`)
      (`/Game/Blueprints/BP_BasePlayerController.UpdateCurrentWeaponState` (`self.OwnerPlayer`) (`self.WeaponState`)))))

(fn `Unequip`
  (params (IsLocal :type Boolean))
  (set `self.Local` IsLocal)
  (set `self.Equipped` false)
  (if (`local.IsLocal`)
    (`self.DisableInput` (`GameplayStatics.GetPlayerController` 0))))

(fn `UserConstructionScript`)

(fn `WeaponAttack`
  (bind _ownerplayer (`self.OwnerPlayer`))
  (bind _returnvalue (`SceneComponent.K2_GetComponentLocation` (`/Game/Blueprints/BP_BaseCharacter.PlayerCamera` (`self.OwnerCharacter`))))
  (bind (_outhit _returnvalue_2) (`KismetSystemLibrary.LineTraceSingle` _returnvalue (+ _returnvalue (* (`KismetMathLibrary.GetForwardVector` (`Controller.GetControlRotation` (`self.OwnerPlayer`))) (`self.GetRange`))) "TraceTypeQuery1" false (`|MakeArray` (`self.OwnerCharacter`) :!type "Actor Object Reference") "ForDuration"))
  (if _returnvalue_2
    (bind (_bblockinghit _binitialoverlap _time _distance _location _impactpoint _normal _impactnormal _physmat _hitactor) (`GameplayStatics.BreakHitResult` _outhit))
    (if (`KismetSystemLibrary.DoesImplementInterface` _hitactor "/Game/BlueprintInterfaces/BI_Game.BI_Game_C")
      (`/Game/Blueprints/BP_BasePlayerController.SERVER_DealDamage` _ownerplayer _hitactor _ownerplayer (make `/Game/Data/F_DamageData` (`self.GetDamage`))))))