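; Base pickup actor that registers itself with a BP_BaseCharacter while that character overlaps its collision.
; Begin overlap stores the locally controlled character and adds the pickup to it; end overlap removes it.
; On pickup, a server event calls an all-clients event, which clears the pickup from each stored character, then destroys the actor.
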(event `self.Collision.OnComponentBeginOverlap`
  (params (OverlappedComponent :type "PrimitiveComponent Object Reference") (OtherActor :type "Actor Object Reference") (OtherComp :type "PrimitiveComponent Object Reference") (OtherBodyIndex :type Integer) (bFromSweep :type Boolean) (SweepResult :type "HitResult Structure (by ref)"))
  ;[0 0 0] Overlapping
  (bind _asbp_base_character (cast `/Game/Blueprints/BP_BaseCharacter` OtherActor))
  (`self.AddPickup` _asbp_base_character))

(event `self.Collision.OnComponentEndOverlap`
  (params (OverlappedComponent :type "PrimitiveComponent Object Reference") (OtherActor :type "Actor Object Reference") (OtherComp :type "PrimitiveComponent Object Reference") (OtherBodyIndex :type Integer))
  ;[0 0 0] Overlapping
  (bind _asbp_base_character (cast `/Game/Blueprints/BP_BaseCharacter` OtherActor))
  (`self.RemovePickup` _asbp_base_character))

(event `PickupItem (OnServer)`
  (params (Player :type "/Game/Blueprints/BP_BasePlayerController Object Reference") (Character :type "/Game/Blueprints/BP_BaseCharacter Object Reference"))
  ;[0 0 0] Pickup on server
  (`self.NETALL_PickupItem`)
  (`self.K2_DestroyActor`))

(event `NETALL_PickupItem`
  ;[0 0 0] Update all clients that might be going to pickup the item
  (`/Engine/EditorBlueprintResources/StandardMacros.IsValid` (`self.Player`)
    (:`Is Valid`
      (`self.RemovePickup` (`self.Player`)))))

(fn `AddPickup`
  (params (Player :type "/Game/Blueprints/BP_BaseCharacter Object Reference"))
  (if (`Pawn.IsLocallyControlled` Player)
    (bind _output_get (set `self.Player` Player))
    (`/Game/Blueprints/BP_BaseCharacter.AddPickup` _output_get self)))

(fn `RemovePickup`
  (params (Player :type "/Game/Blueprints/BP_BaseCharacter Object Reference"))
  (if (== Player (`self.Player`))
    (`/Game/Blueprints/BP_BaseCharacter.RemovePickup` (`self.Player`) self)))

(fn `UserConstructionScript`)