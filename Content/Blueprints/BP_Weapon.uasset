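; BP_Weapon is a hitscan gun actor, driven by WeaponData, that takes Shoot input while equipped.
; Activate fires once or starts a looping timer for full-auto, while Deactivate clears it and locks firing for one shot interval.
; Each shot decrements magazine and reserves, traces from the owner's camera, and sends BI_Game hits to the player's SERVERDealDamage.
; Burst and critical-damage getters exist but go unused here, and no reload is present.
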(event `InputAction|Shoot`
  (params (Key :type "Key Structure"))
  (:`Pressed`
    (set `self.Holding` true)
    (`self.Activate`))
  (:`Released`
    (set `self.Holding` false)
    (`self.Deactivate`)))

(event `Activate`
  (if (and (> (`self.CurrentMag`) 0) (not (`self.Locked`)))
    (`self.Shoot`)
    (if (`self.IsFullAuto`)
      (bind _returnvalue (`KismetSystemLibrary.K2_SetTimerDelegate` (`|CreateDelegate` :!event `Shoot`) (`self.GetShotInterval`) true))
      (set `self.Timer_Shooting` _returnvalue)
      (else
        (`self.Deactivate`)))))

(event `Deactivate`
  (`KismetSystemLibrary.K2_ClearAndInvalidateTimerHandle` (`self.Timer_Shooting`))
  (if (and (not (`self.Locked`)) (`self.Shooting`))
    (set `self.Locked` true)
    (`KismetSystemLibrary.Delay` (`self.GetShotInterval`))
    (set `self.Locked` false)
    (set `self.Shooting` false)
    (if (and (`self.Holding`) (`self.IsFullAuto`))
      (`self.Activate`))))

(event `Shoot`
  (`self.WeaponAttack`)
  (set `self.Shooting` true)
  (`/Engine/EditorBlueprintResources/StandardMacros.DecrementInt` (`self.CurrentMag`)
    (:`  `
      (`/Engine/EditorBlueprintResources/StandardMacros.DecrementInt` (`self.CurrentReserves`)
        (:`  `
          (`KismetSystemLibrary.PrintString` (`KismetStringLibrary.Conv_IntToString` (`self.CurrentMag`)))
          (if (<= (`self.CurrentMag`) 0)
            (`self.Deactivate`)))))))

(fn `Equip`
  (`self.EnableInput` (`GameplayStatics.GetPlayerController` 0))
  (`KismetSystemLibrary.PrintString` "equipped"))

(fn `GetBurstTimes`
  (returns (BurstTimes :type Integer))
  (return (`.BurstTimes_21_09949BCB4DD583CED97EBDBE1BFAE635` (break `/Game/Data/F_Weapon` (`self.WeaponData`)))))

(fn `GetCriticalDamage`
  (returns (ReturnValue :type "Float (double-precision)"))
  (bind (_name _damage _criticalmultiplier) (break `/Game/Data/F_Weapon` (`self.WeaponData`)))
  (return (* _damage _criticalmultiplier)))

(fn `GetDamage`
  (returns (Damage :type "Float (double-precision)"))
  (return (`.Damage_30_DF4AE89E49618FDD61035C86D4ADB3C6` (break `/Game/Data/F_Weapon` (`self.WeaponData`)))))

(fn `GetMagSize`
  (returns (MagSize :type Integer))
  (return (`.MagSize_9_34ACCDEB4D1ECB0A357E81B7846EF234` (break `/Game/Data/F_Weapon` (`self.WeaponData`)))))

(fn `GetMaxReserves`
  (returns (MaxReserves :type Integer))
  (return (`.MaxReserves_12_47E8AF19456C23FB659A86BD9A7F19D6` (break `/Game/Data/F_Weapon` (`self.WeaponData`)))))

(fn `GetRange`
  (returns (Range :type "Float (double-precision)"))
  (return (`.Range_27_5388CA5A4EB0649F4D62F3869F90FA31` (break `/Game/Data/F_Weapon` (`self.WeaponData`)))))

(fn `GetShotInterval`
  (returns (ShotInterval :type "Float (double-precision)"))
  (return (`.ShotInterval_24_D6D9CC57478FA29617F4279E29EB567C` (break `/Game/Data/F_Weapon` (`self.WeaponData`)))))

(fn `GetWeaponName`
  (returns (Name :type Text))
  (return (`.Name_6_EB71841C4C7AC8544E4C0A82C58FCBC2` (break `/Game/Data/F_Weapon` (`self.WeaponData`)))))

(fn `IsBurst`
  (returns (IsBurst :type Boolean))
  (return (`.IsBurst_18_21FF6C044BA0DC0C4CFAAC977BDF4381` (break `/Game/Data/F_Weapon` (`self.WeaponData`)))))

(fn `IsFullAuto`
  (returns (IsAutomatic :type Boolean))
  (return (`.IsAutomatic_16_80C3F7714EF57D7D38E4FAA06EA58A5A` (break `/Game/Data/F_Weapon` (`self.WeaponData`)))))

(fn `Unequip`
  (`self.DisableInput` (`GameplayStatics.GetPlayerController` 0)))

(fn `UserConstructionScript`)

(fn `WeaponAttack`
  (bind _returnvalue (`SceneComponent.K2_GetComponentLocation` (`/Game/Blueprints/BP_BaseCharacter.PlayerCamera` (`self.OwnerCharacter`))))
  (bind (_outhit _returnvalue_2) (`KismetSystemLibrary.LineTraceSingle` _returnvalue (+ _returnvalue (* (`KismetMathLibrary.GetForwardVector` (`Controller.GetControlRotation` (`self.OwnerPlayer`))) (`self.GetRange`))) "TraceTypeQuery1" false (`|MakeArray` (`self.OwnerCharacter`) :!type "Actor Object Reference") "ForDuration"))
  (if _returnvalue_2
    (bind (_bblockinghit _binitialoverlap _time _distance _location _impactpoint _normal _impactnormal _physmat _hitactor) (`GameplayStatics.BreakHitResult` _outhit))
    (if (`KismetSystemLibrary.DoesImplementInterface` _hitactor "/Game/BlueprintInterfaces/BI_Game.BI_Game_C")
      (`/Game/Blueprints/BP_BasePlayerController.SERVER_DealDamage` (`self.OwnerPlayer`) _hitactor (`self.OwnerCharacter`) (make `/Game/Data/F_DamageData` (`self.GetDamage`))))))