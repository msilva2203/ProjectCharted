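; Base game mode for a team-based multiplayer shooter match, managing players, teams, spawning and the return to the lobby when the match ends.
; BeginPlay loads game options, spawners, match-scaled weapon data and persistent pickups; the match starts once all players are ready, and late joiners get the smallest team.
; A one-second timer drives the clock, queued respawn waves and tiered pickup interactability.
; Option handling and winner selection are stubs.
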(event `self.ReceiveBeginPlay`
  ;[0 0 0] Game Instance and Options Handling
  (set `self.Game Instance` (`/Game/BlueprintLibraries/Game.GetGameInstance`))
  (`self.FetchGameOptions`)
  (`self.FindMapData`)
  (`self.FetchWeaponData`)
  (`self.SetupWeaponPickups`))

(event `self.K2_PostLogin`
  (params (NewPlayer :type "PlayerController Object Reference"))
  ;[0 0 0] On Post Login
)

(event `self.HandleStartingNewPlayer`
  (params (NewPlayer :type "PlayerController Object Reference"))
  ;[0 0 0] Handle Starting new Player
  (bind _asbp_base_player_controller (cast `/Game/Blueprints/BP_BasePlayerController` NewPlayer))
  (`KismetArrayLibrary.Array_Add` (`self.Players`) _asbp_base_player_controller)
  (bind _asbp_base_player_state (cast `/Game/Blueprints/BP_BasePlayerState` (`Controller.PlayerState` _asbp_base_player_controller)))
  (`KismetArrayLibrary.Array_Add` (`self.PlayerStates`) _asbp_base_player_state)
  (`/Game/Blueprints/BP_BasePlayerController.CLIENT_SetupPlayer` :`self` _asbp_base_player_controller :`Gamemode` (`self.Gamemode`))
  (`|ExecutionSequence`
    (:`then_0`
      (if (`self.HasStarted`)
        (bind _team (`self.GetSmallestTeam`))
        (`/Game/Blueprints/BP_BasePlayerController.SetTeam` _asbp_base_player_controller _team)
        (else
          (`self.SetPlayerTeams`))))
    (:`then_1`
      (`self.NotifyPlayerStates`))))

(event `self.K2_OnLogout`
  (params (ExitingController :type "Controller Object Reference"))
  ;[0 0 0] Player Logout
  (bind _asbp_base_player_controller (cast `/Game/Blueprints/BP_BasePlayerController` ExitingController))
  (if (`KismetArrayLibrary.Array_Contains` (`self.Players`) _asbp_base_player_controller)
    (bind _returnvalue (`KismetArrayLibrary.Array_RemoveItem` (`self.Players`) _asbp_base_player_controller))
    (if _returnvalue
      (bind _asbp_base_player_state (cast `/Game/Blueprints/BP_BasePlayerState` (`Controller.PlayerState` _asbp_base_player_controller)))
      (`KismetArrayLibrary.Array_RemoveItem` (`self.PlayerStates`) _asbp_base_player_state))))

(event `StartMatchTimer`
  ;[0 0 0] Match Timer Handle
  (bind _returnvalue (`KismetSystemLibrary.K2_SetTimer` null "OnMatchTimerUpdate" 1.0 true))
  (set `self.Timer_Match` _returnvalue))

(fn `AddPlayerToDeadList`
  (params (Player :type "/Game/Blueprints/BP_BasePlayerController Object Reference"))
  (`KismetArrayLibrary.Array_Add` (`self.Players_Dead`) Player)
  (`KismetSystemLibrary.PrintString` "Added player to dead list"))

(fn `AddPlayerToDeadQueue`
  (params (Player :type "/Game/Blueprints/BP_BasePlayerController Object Reference"))
  (`KismetArrayLibrary.Array_Add` (`self.Players_DeadQueue`) Player)
  (`KismetSystemLibrary.PrintString` "Added player to dead queue"))

(fn `EndMatch`
  (params (HasWinningTeam :type Boolean))
  (if (not HasWinningTeam)
    (bind _team (`self.FindWinningTeam`))
    (`self.SetWinningTeam` _team))
  (`KismetSystemLibrary.PrintString` (`KismetStringLibrary.Concat_StrStr` (`|GetEnumeratorNameAsString` (`self.GetWinningTeam`)) " won the game!"))
  (`self.ReturnToLobby`))

(fn `FetchGameOptions`
  (for _array_element (`/Game/Blueprints/BP_GameInstance.GetGameOptions` (`self.Game Instance`))
    (bind (_gameoption_name _gameoption_description _gameoption_options _gameoption_selected) (break `/Game/Data/F_GameOption` _array_element))
    (`self.HandleGameOptions` (`KismetTextLibrary.Conv_TextToString` (`KismetTextLibrary.TextToLower` _gameoption_name)) _gameoption_selected)))

(fn `FetchWeaponData`
  (locals (TEMP_Data :type "/Game/Data/F_Weapon Structure"))
  (bind (_damagemultiplier _criticaldamagemultiplier _maxreservesmultiplier _magsizemultiplier) (break `/Game/Data/F_CombatOptions` (`.Match_CombatOptions_20_4A7E71484FD863B93370609F717DB04F` (break `/Game/Data/F_Match` (`self.MatchData`)))))
  (bind _outrownames (`DataTableFunctionLibrary.GetDataTableRowNames` "/Game/Data/DT_Weapons.DT_Weapons"))
  (for _array_element _outrownames
    (bind _returnvalue (`|GetDataTableRow` "/Game/Data/DT_Weapons.DT_Weapons" _array_element)
      (:`then`
        (bind _output_get (set `local.TEMP_Data` _returnvalue))
        (bind (_name _weapon _equipment _tier _damage _criticalmultiplier _magsize _maxreserves _shotinterval _range _isautomatic _isburst _bursttimes _state) (break `/Game/Data/F_Weapon` _returnvalue))
        (bind (_currentmag _currentreserves) (break `/Game/Data/F_WeaponState` _state))
        (bind _structout (setmembers `/Game/Data/F_Weapon` :`StructRef` _output_get :`Damage` (* _damage _damagemultiplier) :`CriticalMultiplier` (* _criticalmultiplier _criticaldamagemultiplier) :`MagSize` (`KismetMathLibrary.FTrunc` (* (`KismetMathLibrary.Conv_IntToDouble` _magsize) _maxreservesmultiplier)) :`MaxReserves` (`KismetMathLibrary.FTrunc` (* (`KismetMathLibrary.Conv_IntToDouble` _maxreserves) _magsizemultiplier)) :`State` (make `/Game/Data/F_WeaponState` (`KismetMathLibrary.FTrunc` (* (`KismetMathLibrary.Conv_IntToDouble` _currentmag) _magsizemultiplier)) (`KismetMathLibrary.FTrunc` (* (`KismetMathLibrary.Conv_IntToDouble` _currentreserves) _maxreservesmultiplier)))))
        (`KismetArrayLibrary.Array_Add` (`self.Weapons`) _structout)))))

(fn `FindAvailableSpawner`
  (params (RequestedTeam :type "/Game/Data/E_Team Enum" :default "NewEnumerator0"))
  (returns (`Array Element` :type "/Game/Blueprints/BP_PlayerSpawner Object Reference"))
  (locals (TEMP_Found :type Boolean) (TEMP_Spawners :type "Array of /Game/Blueprints/BP_PlayerSpawner Object Reference"))
  (for _array_element (`self.Spawners`)
    (bind _team (`/Game/BlueprintInterfaces/BI_Game.GetTeam` _array_element))
    (if (and (`|EnumEquality` _team (`local.RequestedTeam`)) (`/Game/Blueprints/BP_PlayerSpawner.IsAvailable` _array_element))
      (`KismetArrayLibrary.Array_Add` (`local.TEMP_Spawners`) _array_element)
      (set `local.TEMP_Found` true)))
  (if (not (`local.TEMP_Found`))
    (for _array_element_2 (`self.Spawners`)
      (if (`/Game/Blueprints/BP_PlayerSpawner.IsAvailable` _array_element_2)
        (`KismetArrayLibrary.Array_Add` (`local.TEMP_Spawners`) _array_element_2))))
  (return (`KismetArrayLibrary.Array_Random` (`local.TEMP_Spawners`))))

(fn `FindMapData`
  (bind _outactors (`GameplayStatics.GetAllActorsOfClass` "/Game/Blueprints/BP_PlayerSpawner.BP_PlayerSpawner_C"))
  (set `self.Spawners` _outactors))

(fn `FindWinningTeam`
  (returns (Team :type "/Game/Data/E_Team Enum"))
  (return "NewEnumerator0"))

(fn `GetDefaultWeaponState`
  (params (Weapon :type "/Game/Data/E_Weapon Enum" :default "NewEnumerator0"))
  (returns (State :type "/Game/Data/F_WeaponState Structure"))
  (bind _weapondata (`self.GetWeaponData` Weapon))
  (return (`.State_41_442C029945012BF511E2AB867B29433C` (break `/Game/Data/F_Weapon` _weapondata))))

(fn `GetMatchData`
  (returns (MatchData :type "/Game/Data/F_Match Structure"))
  (return (`self.MatchData`)))

(fn `GetRespawnInterval`
  (returns (Match_RespawnInterval :type Integer))
  (return (`.Match_RespawnInterval_5_46B9472F4918C137550E30BC745569C8` (break `/Game/Data/F_Match` (`self.MatchData`)))))

(fn `GetSmallestTeam`
  (returns (Team :type "/Game/Data/E_Team Enum"))
  (locals (TEMP_Teams :type "Array of Integer") (TEMP_Smallest :type Integer) (TEMP_Team :type "/Game/Data/E_Team Enum"))
  (for _ (range 1 (+ (`self.NumTeams`) 1))
    (`KismetArrayLibrary.Array_Add` (`local.TEMP_Teams`)))
  (for _array_element (`self.Players`)
    (bind _team (`/Game/BlueprintInterfaces/BI_Game.GetTeam` _array_element))
    (if (`|EnumInequality` _team "NewEnumerator0")
      (`/Engine/EditorBlueprintResources/StandardMacros.IncrementInt` (`|GetArrayItem` (`local.TEMP_Teams`) (- (`KismetMathLibrary.Conv_ByteToInt` _team) 1)))))
  (set `local.TEMP_Smallest` (`|GetArrayItem` (`local.TEMP_Teams`)))
  (set `local.TEMP_Team` "NewEnumerator1")
  (for (_array_element_2 _array_index) (`local.TEMP_Teams`)
    (if (<= _array_element_2 (`local.TEMP_Smallest`))
      (set `local.TEMP_Team` (cast `/Game/Data/E_Team` (`KismetMathLibrary.Conv_IntToByte` (+ _array_index 1))))
      (set `local.TEMP_Smallest` _array_element_2)))
  (return (`local.TEMP_Team`)))

(fn `GetTime`
  (returns (Match_Time :type Integer))
  (return (`.Match_Time_3_96A8A20B4D43F5304E2AD496BEEF8B17` (break `/Game/Data/F_Match` (`self.MatchData`)))))

(fn `GetWeaponData`
  (params (Weapon :type "/Game/Data/E_Weapon Enum" :default "NewEnumerator0"))
  (returns (WeaponData :type "/Game/Data/F_Weapon Structure"))
  (if (not (`|EnumEquality` Weapon "NewEnumerator0"))
    (return (`|GetArrayItem` (`self.Weapons`) (- (`KismetMathLibrary.Conv_ByteToInt` (`local.Weapon`)) 1)))
    (else
      (return))))

(fn `GetWeaponTier`
  (params (Weapon :type "/Game/Data/E_Weapon Enum" :default "NewEnumerator0"))
  (returns (Tier :type "/Game/Data/E_WeaponTier Enum"))
  (for _array_element (`self.Weapons`)
    (bind (_name _weapon _equipment _tier) (break `/Game/Data/F_Weapon` _array_element))
    (if (`|EnumEquality` _weapon (`local.Weapon`))
      (return _tier))))

(fn `GetWinningTeam`
  (returns (ReturnValue :type "/Game/Data/E_Team Enum"))
  (return (`self.WinningTeam`)))

(fn `HandleGameOptions`
  (params (Option :type String) (SelectedOption :type Integer)))

(fn `NotifyPlayerStates`
  (for _array_element (`self.Players`)
    (`/Game/Blueprints/BP_BasePlayerController.SetPlayerStates` _array_element (`self.PlayerStates`))))

(fn `OnMatchTimerUpdate`
  (locals (TEMP_Respawn :type Integer :default 0))
  (bind (_match_time _match_respawninterval _match_canrespawn _match_friendlyfire _match_userespawnwaves _match_weaponpickups) (break `/Game/Data/F_Match` (`self.MatchData`)))
  (bind (_tier1 _tier2 _tier3) (break `/Game/Data/F_WeaponPickupOption` _match_weaponpickups))
  (bind (_interactable _time) (break `/Game/Data/F_WeaponPickupState` _tier1))
  (bind (_interactable_2 _time_2) (break `/Game/Data/F_WeaponPickupState` _tier2))
  (bind (_interactable_3 _time_3) (break `/Game/Data/F_WeaponPickupState` _tier3))
  (`|ExecutionSequence`
    (:`then_0`
      (bind _result (`/Engine/EditorBlueprintResources/StandardMacros.DecrementInt` _match_time)
        (:`  `
          (`self.OnTimeUpdate` _result)
          (if (<= _match_time 0)
            (`self.EndMatch` false)))))
    (:`then_1`
      (if (`self.UseRespawnWaves`)
        (set `local.TEMP_Respawn` (mod _match_time _match_respawninterval))
        (`|ExecutionSequence`
          (:`then_0`
            (if (== 0 (`local.TEMP_Respawn`))
              (`self.SpawnCharacters` (`self.Players_Dead`))
              (set `self.Players_Dead` (`self.Players_DeadQueue`))
              (`KismetArrayLibrary.Array_Clear` (`self.Players_DeadQueue`))))
          (:`then_1`
            (`self.OnRespawnTimeUpdate` (`local.TEMP_Respawn`))))))
    (:`then_2`
      (`|ExecutionSequence`
        (:`then_0`
          (if (== (mod _match_time _time) 0)
            (`self.Set Weapon Pickups` "NewEnumerator0" _interactable)))
        (:`then_1`
          (if (== (mod _match_time _time_2) 0)
            (`self.Set Weapon Pickups` "NewEnumerator1" _interactable_2)))
        (:`then_2`
          (if (== (mod _match_time _time_3) 0)
            (`self.Set Weapon Pickups` "NewEnumerator2" _interactable_3)))))))

(fn `OnPlayerReady`
  (params (Player :type "/Game/Blueprints/BP_BasePlayerController Object Reference"))
  (bind _array (`|MakeArray` Player))
  (bind _returnvalue (`/Game/Blueprints/BP_GameInstance.GetNumPlayers` (`self.Game Instance`)))
  (if (`KismetArrayLibrary.Array_Contains` (`self.Players`) Player)
    (if (not (`self.HasStarted`))
      (bind _result (`/Engine/EditorBlueprintResources/StandardMacros.IncrementInt` (`self.NumPlayersReady`))
        (:`  `
          (`KismetSystemLibrary.PrintString` (`KismetStringLibrary.Concat_StrStr` (`KismetStringLibrary.Conv_IntToString` _result) "/" (`KismetStringLibrary.Conv_IntToString` _returnvalue)))
          (if (>= _result _returnvalue)
            (`self.StartMatch`))))
      (else
        (`self.StartPlayers` _array)
        (`self.SpawnCharacters` _array true)))))

(fn `Remove Character`
  (params (PlayerToKill :type "/Game/Blueprints/BP_BasePlayerController Object Reference"))
  (bind _returnvalue (`KismetArrayLibrary.Array_RemoveItem` (`self.Characters`) (`/Game/Blueprints/BP_BasePlayerController.PlayerCharacter` PlayerToKill)))
  (if _returnvalue
    (`Controller.UnPossess` (`local.PlayerToKill`))))

(fn `ReturnToLobby`
  (`KismetSystemLibrary.ExecuteConsoleCommand` "servertravel L_Lobby?game=LOBBY" (`GameplayStatics.GetPlayerController` 0)))

(fn `Set Weapon Pickups`
  (params (Tier :type "/Game/Data/E_WeaponTier Enum" :default "NewEnumerator0") (Interactable :type Boolean))
  (for _array_element (`self.Pickups_Weapons`)
    (if (or (`|EnumEquality` (`/Game/Blueprints/BP_Pickup_Weapon.GetWeaponTier` _array_element) (`local.Tier`)) (`|EnumEquality` Tier "NewEnumerator3"))
      (`/Game/Blueprints/BP_BasePickup.SetIsInteractable` _array_element (`local.Interactable`)))))

(fn `SetFriendlyFire`
  (params (NewValue :type Boolean))
  (`|VariableSetRef` (`.Match_FriendlyFire_11_B573F7CF461C62F178F62EBEDAA9F58E` (break `/Game/Data/F_Match` (`self.MatchData`))) NewValue))

(fn `SetPlayerTeams`
  (for (_array_element _array_index) (`self.Players`)
    (`/Game/Blueprints/BP_BasePlayerController.SetTeam` _array_element (cast `/Game/Data/E_Team` (`KismetMathLibrary.Conv_IntToByte` (+ (mod _array_index (`self.NumTeams`)) 1))))))

(fn `SetRespawnInterval`
  (params (Value :type Integer))
  (`|VariableSetRef` (`.Match_RespawnInterval_5_46B9472F4918C137550E30BC745569C8` (break `/Game/Data/F_Match` (`self.MatchData`))) Value))

(fn `SetTime`
  (params (Value :type Integer))
  (`|VariableSetRef` (`.Match_Time_3_96A8A20B4D43F5304E2AD496BEEF8B17` (break `/Game/Data/F_Match` (`self.MatchData`))) Value))

(fn `SetupWeaponPickups`
  (bind (_tier1 _tier2 _tier3) (break `/Game/Data/F_WeaponPickupOption` (`.Match_WeaponPickups_17_232E1B0B443B67DFBB53D09D2571B478` (break `/Game/Data/F_Match` (`self.MatchData`)))))
  (bind _outactors (`GameplayStatics.GetAllActorsOfClass` "/Game/Blueprints/BP_Pickup_Weapon.BP_Pickup_Weapon_C"))
  (for _array_element _outactors
    (if (`/Game/Blueprints/BP_BasePickup.IsPersistent` _array_element)
      (`KismetArrayLibrary.Array_Add` (`self.Pickups_Weapons`) _array_element)
      (`/Game/Blueprints/BP_Pickup_Weapon.SetWeaponState` _array_element (`self.GetDefaultWeaponState` (`/Game/Blueprints/BP_Pickup_Weapon.GetWeapon` _array_element)))
      (bind _tier (`self.GetWeaponTier` "NewEnumerator0"))
      (`/Game/Blueprints/BP_Pickup_Weapon.SetWeaponTier` _array_element _tier)
      (switch `/Game/Data/E_WeaponTier` _tier
        (:`NewEnumerator0`
          (`/Game/Blueprints/BP_BasePickup.SetIsInteractable` _array_element (`.Interactable_3_6E18950046C538CACA2034A68C5216F4` (break `/Game/Data/F_WeaponPickupState` _tier1))))
        (:`NewEnumerator1`
          (`/Game/Blueprints/BP_BasePickup.SetIsInteractable` _array_element (`.Interactable_3_6E18950046C538CACA2034A68C5216F4` (break `/Game/Data/F_WeaponPickupState` _tier2))))
        (:`NewEnumerator2`
          (`/Game/Blueprints/BP_BasePickup.SetIsInteractable` _array_element (`.Interactable_3_6E18950046C538CACA2034A68C5216F4` (break `/Game/Data/F_WeaponPickupState` _tier3))))))))

(fn `SetUseRespawnWaves`
  (params (NewValue :type Boolean))
  (`|VariableSetRef` (`.Match_UseRespawnWaves_14_D84DD8CB4C34EAAE21F78C963DF01904` (break `/Game/Data/F_Match` (`self.MatchData`))) NewValue))

(fn `SetWinningTeam`
  (params (Team :type "/Game/Data/E_Team Enum" :default "NewEnumerator0"))
  (set `self.WinningTeam` Team))

(fn `SpawnCharacters`
  (params (Players :type "Array of /Game/Blueprints/BP_BasePlayerController Object Reference") (UsePlayerTeam :type Boolean))
  (locals (TEMP_NewCharacters :type "Array of /Game/Blueprints/BP_BaseCharacter Object Reference"))
  (if (not (`KismetArrayLibrary.Array_IsEmpty` Players))
    (for _array_element Players
      (bind _team (`/Game/BlueprintInterfaces/BI_Game.GetTeam` _array_element))
      (bind _character (`/Game/Blueprints/BP_PlayerSpawner.SpawnPlayer` (`self.FindAvailableSpawner` (select `bool` (`local.UsePlayerTeam`) :`false` "NewEnumerator0" :`true` _team)) _array_element))
      (`KismetArrayLibrary.Array_Add` (`self.Characters`) _character)
      (`KismetArrayLibrary.Array_Add` (`local.TEMP_NewCharacters`) _character))
    (for _array_element_2 (`local.TEMP_NewCharacters`)
      (`/Game/Blueprints/BP_BaseCharacter.SERVER_SetupCharacter` _array_element_2))))

(fn `StartMatch`
  (`self.StartPlayers` (`self.Players`))
  (`self.SpawnCharacters` (`self.Players`) true)
  (`self.StartMatchTimer`)
  (set `self.HasStarted` true)
  (`KismetSystemLibrary.PrintString` "Match Started"))

(fn `StartPlayers`
  (params (Players :type "Array of /Game/Blueprints/BP_BasePlayerController Object Reference"))
  (for _array_element Players
    (`/Game/Blueprints/BP_BasePlayerController.CLIENT_StartPlayer` _array_element)))

(fn `UserConstructionScript`)

(fn `UseRespawnWaves`
  (returns (ReturnValue :type Boolean))
  (return (`/Game/BlueprintLibraries/Match.UseRespawnWaves` (`self.MatchData`))))