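; Base networked character for a team-based shooter, handling movement, aiming, health, weapons and item pickup.
; Local action state changes mirror through the server to other clients, while primary/secondary weapons are server-spawned and equipped via RepNotifies.
; Server damage respects friendly fire, credits kills and assists, and starts timed regeneration, with desaturation and heartbeat as health feedback.
; A local timer selects the nearest pickup for the HUD; remote characters get team-colored name tags.
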(event `self.ReceiveBeginPlay`
  (`self.SetActionState` (`self.ActionState`) true))

(event `self.ReceiveTick`
  (params (DeltaSeconds :type "Float (single-precision)"))
  (`self.Tick_Client`)
  (`self.PrintDebugInfo`))

(event `self.DamageActor`
  (params (Instigator :type "Actor Object Reference") (`Damage Data` :type "/Game/Data/F_DamageData Structure"))
  (`self.SERVER_ReceiveDamage` Instigator `Damage Data`))

(event `self.AddKill`
  (`self.OnKill`)
  (`self.CLIENT_OnKill`))

(event `self.AddAssist`
  (`KismetSystemLibrary.PrintString` "Assist"))

(event `InputAxis|MoveForward`
  (params (AxisValue :type "Float (single-precision)"))
  (bind (_returnvalue_roll _returnvalue_pitch _returnvalue_yaw) (`KismetMathLibrary.BreakRotator` (`self.GetControlRotation`)))
  (`self.AddMovementInput` (`KismetMathLibrary.GetForwardVector` (`KismetMathLibrary.MakeRotator` 0.0 0.0 _returnvalue_yaw)) AxisValue))

(event `InputAxis|LookUp`
  (params (AxisValue :type "Float (single-precision)"))
  (`self.AddControllerPitchInput` AxisValue))

(event `InputAxis|Turn`
  (params (AxisValue :type "Float (single-precision)"))
  (`self.AddControllerYawInput` AxisValue))

(event `InputAxis|MoveRight`
  (params (AxisValue :type "Float (single-precision)"))
  (bind (_returnvalue_roll _returnvalue_pitch _returnvalue_yaw) (`KismetMathLibrary.BreakRotator` (`self.GetControlRotation`)))
  (`self.AddMovementInput` (`KismetMathLibrary.GetRightVector` (`KismetMathLibrary.MakeRotator` 0.0 0.0 _returnvalue_yaw)) AxisValue))

(event `InputAction|Aim`
  (params (Key :type "Key Structure"))
  (:`Pressed`
    (`self.SetActionState` "NewEnumerator2" true))
  (:`Released`
    (`self.SetActionState` "NewEnumerator1" true)))

(event `InputAction|Interact`
  (params (Key :type "Key Structure"))
  (:`Pressed`
    (`/Engine/EditorBlueprintResources/StandardMacros.IsValid` (`self.CurrentPickup`)
      (:`Is Valid`
        (`/Game/Blueprints/BP_BasePlayerController.SERVER_PickupItem` (`self.PlayerController`) (`self.CurrentPickup`))))))

(event `InputAction|Primary`
  (params (Key :type "Key Structure"))
  (:`Pressed`
    (if (`|EnumInequality` (`self.CurrentEquipment`) "NewEnumerator1")
      (`self.SERVER_SetEquipment` "NewEnumerator1"))))

(event `InputAction|Secondary`
  (params (Key :type "Key Structure"))
  (:`Pressed`
    (if (`|EnumInequality` (`self.CurrentEquipment`) "NewEnumerator2")
      (`self.SERVER_SetEquipment` "NewEnumerator2"))))

(event `SERVER_SetupCharacter`
  ;[0 0 0] Player Character Network Setup
  (`self.NETALL_SetupCharacter`)
  (set `self.Base Gamemode` (`/Game/BlueprintLibraries/Game.GetBaseGamemode`))
  (bind _asbp_base_player_controller (cast `/Game/Blueprints/BP_BasePlayerController` (`self.GetController`)))
  (set `self.PlayerController` _asbp_base_player_controller)
  (`self.SERVER_PickupWeapon` "NewEnumerator2" "NewEnumerator2" (struct) true)
  (`self.SERVER_PickupWeapon` "NewEnumerator1" "NewEnumerator1" (struct) true))

(event `NETALL_SetupCharacter`
  ;[0 0 0] Player Character Network Setup
  (if (`self.IsLocallyControlled`)
    (`self.Setup_Local`)
    (else
      (`KismetSystemLibrary.Delay` 1.0)
      (`self.Setup_NotLocal`))))

(event `SERVER_SetActionState`
  (params (NewState :type "/Game/Data/E_ActionState Enum" :default "NewEnumerator0"))
  ;[0 0 0] Action State Replication
  (bind _state (`self.SetActionState` NewState))
  (`self.NETALL_SetActionState` _state))

(event `NETALL_SetActionState`
  (params (NewState :type "/Game/Data/E_ActionState Enum" :default "NewEnumerator0"))
  ;[0 0 0] Action State Replication
  (if (and (not (`KismetSystemLibrary.IsServer`)) (not (`self.IsLocallyControlled`)))
    (`self.SetActionState` NewState)))

(event `SERVER_ReceiveDamage`
  (params (Instigator :type "Actor Object Reference") (`Damage Data` :type "/Game/Data/F_DamageData Structure"))
  ;[0 0 0] Health handling
  (`self.ReceiveDamage` Instigator `Damage Data`))

(event `SERVER_StartHealthRegen`
  ;[0 0 0] Health handling
  (bind _returnvalue (`KismetSystemLibrary.K2_SetTimerDelegate` (delegate `OnStartRegen`) (`self.RegenStartTime`)))
  (set `self.Timer_HealthRegenStart` _returnvalue)
  (set `self.RegenOffset` (/ (- (`self.MaxHealth`) (`self.Health`)) (`self.HealthRegenTicks`)))
  (set `self.RegenCount` 0)
  (`KismetSystemLibrary.K2_ClearAndInvalidateTimerHandle` (`self.Timer_HealthRegen`)))

(event `OnStartRegen`
  ;[0 0 0] Health handling
  (bind _returnvalue (`KismetSystemLibrary.K2_SetTimerDelegate` (delegate `OnHealthRegen`) (/ (`self.RegenTime`) (`KismetMathLibrary.Conv_IntToDouble` (`self.HealthRegenTicks`))) true))
  (set `self.Timer_HealthRegen` _returnvalue))

(event `OnHealthRegen`
  (bind _regencount (`self.RegenCount`))
  ;[0 0 0] Health handling
  (`/Engine/EditorBlueprintResources/StandardMacros.IncrementInt` _regencount
    (:`  `
      (if (== _regencount (`self.HealthRegenTicks`))
        (set `self.Health` (`self.MaxHealth`))
        (`KismetSystemLibrary.K2_ClearAndInvalidateTimerHandle` (`self.Timer_HealthRegen`))
        (set `self.KillingInstigator` null)
        (set `self.AssistingInstigator` null)
        (else
          (set `self.Health` (+ (`self.Health`) (`self.RegenOffset`)))))
      (`self.CLIENT_Updatehealth` (`self.Health`)))))

(event `CLIENT_Updatehealth`
  (params (Health :type "Float (double-precision)"))
  ;[0 0 0] Health handling
  (bind _output_get (set `self.Health` Health))
  (`self.UpdateHealthFeedback` (/ _output_get (`self.MaxHealth`))))

(event `NETALL_OnDeath`
  ;[0 0 0] Health handling
  (if (`self.IsLocallyControlled`)
    (`self.UpdateHealthFeedback` 1.0)
    (`AudioComponent.Stop` (`self.AUDIO_Heartbeat`))
    (else
      (`/Game/UserInterface/Gameplay/Components/WBP_PlayerTag.SwitchToDeath` (`self.PlayerTag`)))))

(event `SERVER_PickupWeapon`
  (params (Weapon :type "/Game/Data/E_Weapon Enum" :default "NewEnumerator0") (Equipment :type "/Game/Data/E_Equipment Enum" :default "NewEnumerator0") (WeaponState :type "/Game/Data/F_WeaponState Structure") (UseDefaultWeaponState :type Boolean))
  (`self.PickupWeapon (OnServer)` Weapon Equipment (select `bool` UseDefaultWeaponState :`false` WeaponState :`true` (`/Game/Blueprints/BP_BaseGamemode.GetDefaultWeaponState` (`self.Base Gamemode`) Weapon))))

(event `CLIENT_OnKill`)

(event `SERVER_SetEquipment`
  (params (NewEquipment :type "/Game/Data/E_Equipment Enum" :default "NewEnumerator0"))
  (bind _output_get (set `self.CurrentEquipment` NewEquipment))
  (`self.CLIENT_SetEquipment` _output_get))

(event `CLIENT_SetEquipment`
  (params (NewEquipment :type "/Game/Data/E_Equipment Enum" :default "NewEnumerator0"))
  (bind _output_get (set `self.CurrentEquipment` NewEquipment))
  (`self.EquipWeapon` _output_get true))

(event `SERVER_DropEquipment`
  (params (Equipment :type "/Game/Data/E_Equipment Enum" :default "NewEnumerator0"))
  (bind (_weapon _isvalid) (`self.GetEquipment` Equipment))
  (if _isvalid
    (bind _returnvalue (`|SpawnActorFromClass` "/Game/Blueprints/BP_Pickup_Weapon.BP_Pickup_Weapon_C" (`self.GetTransform`) "AlwaysSpawn" "OverrideRootScale" null (`/Game/Blueprints/BP_BaseWeapon.GetWeaponEnum` _weapon) false null))
    (`/Game/Blueprints/BP_Pickup_Weapon.SetWeaponState` _returnvalue (`/Game/Blueprints/BP_BaseWeapon.WeaponState` _weapon))
    (`self.K2_DestroyActor` _weapon)))

(event `StartPickupTimer`
  ;[0 0 0] Timers
  (bind _returnvalue (`KismetSystemLibrary.K2_SetTimerDelegate` (delegate `EVENT_OnPickupEvaluation`) 0.05 true))
  (set `self.Timer_Pickups` _returnvalue))

(event `EVENT_OnPickupEvaluation`
  ;[0 0 0] Timers
  (`self.HandlePickups`))

(fn `AddPickup`
  (params (Pickup :type "/Game/Blueprints/BP_BasePickup Object Reference"))
  (`KismetArrayLibrary.Array_Add` (`self.Pickups`) Pickup))

(fn `CreatePlayerTag`
  (params (Color :type "LinearColor Structure"))
  (bind _playertag (`self.PlayerTag`))
  (bind _returnvalue (`|CreateWidget` "/Game/UserInterface/Gameplay/Components/WBP_PlayerTag.WBP_PlayerTag_C" (`GameplayStatics.GetPlayerController` 0)))
  (bind _output_get (set `self.PlayerTag` _returnvalue))
  (`/Game/UserInterface/Gameplay/Components/WBP_PlayerTag.UpdatePlayerTag` _output_get (`KismetTextLibrary.Conv_StringToText` (`PlayerState.GetPlayerName` (`self.PlayerState`))) Color)
  (`WidgetComponent.SetWidget` (`self.WC_PlayerTag`) _playertag)
  (`/Game/UserInterface/Gameplay/Components/WBP_PlayerTag.SwitchToAlive` _playertag))

(fn `EquipWeapon`
  (params (Equipment :type "/Game/Data/E_Equipment Enum" :default "NewEnumerator0") (IsLocal :type Boolean))
  (bind _weapon_primary (`self.Weapon_Primary`))
  (bind _islocal (`local.IsLocal`))
  (bind _weapon_secondary (`self.Weapon_Secondary`))
  (bind _islocal_2 (`local.IsLocal`))
  (`|ExecutionSequence`
    (:`then_0`
      (switch `/Game/Data/E_Equipment` (`local.Equipment`)
        (:`NewEnumerator0`
          (return))
        (:`NewEnumerator1`
          (`|ExecutionSequence`
            (:`then_0`
              (`/Engine/EditorBlueprintResources/StandardMacros.IsValid` (`self.Weapon_Primary`)
                (:`Is Valid`
                  (`/Game/Blueprints/BP_BaseWeapon.Equip` (`self.Weapon_Primary`) _islocal))
                (:`Is Not Valid`
                  (return))))
            (:`then_1`
              (`/Engine/EditorBlueprintResources/StandardMacros.IsValid` _weapon_secondary
                (:`Is Valid`
                  (`/Game/Blueprints/BP_BaseWeapon.Unequip` _weapon_secondary _islocal))))))
        (:`NewEnumerator2`
          (`|ExecutionSequence`
            (:`then_0`
              (`/Engine/EditorBlueprintResources/StandardMacros.IsValid` (`self.Weapon_Secondary`)
                (:`Is Valid`
                  (`/Game/Blueprints/BP_BaseWeapon.Equip` (`self.Weapon_Secondary`) _islocal_2))
                (:`Is Not Valid`
                  (return))))
            (:`then_1`
              (`/Engine/EditorBlueprintResources/StandardMacros.IsValid` _weapon_primary
                (:`Is Valid`
                  (`/Game/Blueprints/BP_BaseWeapon.Unequip` _weapon_primary _islocal_2))))))))
    (:`then_1`
      (`TextRenderComponent.K2_SetText` (`self.TextRender`) (`/Game/Blueprints/BP_BaseWeapon.GetWeaponName` (`self.GetEquippedWeapon`))))))

(fn `GetActionState`
  (returns (ActionState :type "/Game/Data/E_ActionState Enum"))
  (return (`self.ActionState`)))

(fn `GetAssists`
  (returns (Assists :type Integer))
  (bind _assists (message `/Game/BlueprintInterfaces/BI_Game.GetAssists` (`self.PlayerState`)))
  (return _assists))

(fn `GetDeaths`
  (returns (Deaths :type Integer))
  (bind _deaths (message `/Game/BlueprintInterfaces/BI_Game.GetDeaths` (`self.PlayerState`)))
  (return _deaths))

(fn `GetEquipment`
  (params (Equipment :type "/Game/Data/E_Equipment Enum" :default "NewEnumerator0"))
  (returns (Weapon :type "/Game/Blueprints/BP_BaseWeapon Object Reference") (IsValid :type Boolean))
  (bind _returnvalue (select `/Game/Data/E_Equipment` (`local.Equipment`) :`NewEnumerator1` (`self.Weapon_Primary`) :`NewEnumerator2` (`self.Weapon_Secondary`)))
  (return _returnvalue (`KismetSystemLibrary.IsValid` _returnvalue)))

(fn `GetEquippedWeapon`
  (returns (Weapon :type "/Game/Blueprints/BP_BaseWeapon Object Reference"))
  (bind _weapon_primary (`self.Weapon_Primary`))
  (return (select `/Game/Data/E_Equipment` (`self.CurrentEquipment`) :`NewEnumerator0` _weapon_primary :`NewEnumerator1` _weapon_primary :`NewEnumerator2` (`self.Weapon_Secondary`))))

(fn `GetFocusLocation`
  (returns (Location :type "Vector Structure"))
  (return (`self.K2_GetActorLocation`)))

(fn `GetKills`
  (returns (Kills :type Integer))
  (bind _kills (message `/Game/BlueprintInterfaces/BI_Game.GetKills` (`self.PlayerState`)))
  (return _kills))

(fn `GetScore`
  (returns (Score :type Integer))
  (bind _score (message `/Game/BlueprintInterfaces/BI_Game.GetScore` (`self.PlayerState`)))
  (return _score))

(fn `GetTeam`
  (returns (Team :type "/Game/Data/E_Team Enum"))
  (bind _team (message `/Game/BlueprintInterfaces/BI_Game.GetTeam` (`self.PlayerState`)))
  (return _team))

(fn `HandlePickups`
  (locals (TEMP_Distance :type "Float (double-precision)" :default 0.0) (TEMP_Pickup :type "/Game/Blueprints/BP_BasePickup Object Reference") (TEMP_ItDistance :type "Float (double-precision)" :default 0.0))
  (bind _output (`|GetArrayItem` (`self.Pickups`)))
  (if (`KismetArrayLibrary.Array_IsEmpty` (`self.Pickups`))
    (`self.SetCurrentPickup` null)
    (else
      (set `local.TEMP_Distance` (`KismetMathLibrary.Vector_Distance` (`self.K2_GetActorLocation`) (`self.K2_GetActorLocation` _output)))
      (set `local.TEMP_Pickup` _output)
      (for _array_element (`self.Pickups`)
        (bind _output_get (set `local.TEMP_ItDistance` (`KismetMathLibrary.Vector_Distance` (`self.K2_GetActorLocation` _array_element) (`self.K2_GetActorLocation`))))
        (if (<= _output_get (`local.TEMP_Distance`))
          (set `local.TEMP_Distance` (`local.TEMP_ItDistance`))
          (set `local.TEMP_Pickup` _array_element)))
      (`self.SetCurrentPickup` (`local.TEMP_Pickup`)))))

(fn `IsAiming`
  (returns (ReturnValue :type Boolean))
  (return (`|EnumEquality` (`self.ActionState`) "NewEnumerator2")))

(fn `IsWalking`
  (returns (ReturnValue :type Boolean))
  (return (`|EnumEquality` (`self.ActionState`) "NewEnumerator1")))

(fn `OnRep_CurrentEquipment`
  (if (not (`self.IsLocallyControlled`))
    (`self.EquipWeapon` (`self.CurrentEquipment`))))

(fn `OnRep_Weapon_Primary`
  (if (`self.IsLocallyControlled`)
    (`self.SERVER_SetEquipment` "NewEnumerator1")
    (`KismetSystemLibrary.PrintString` "Primary weapon is ready to be used in this client")
    (else
      (`self.EquipWeapon` (`self.CurrentEquipment`)))))

(fn `OnRep_Weapon_Secondary`
  (if (`self.IsLocallyControlled`)
    (`self.SERVER_SetEquipment` "NewEnumerator2")
    (else
      (`self.EquipWeapon` (`self.CurrentEquipment`)))))

(fn `PickupWeapon (OnServer)`
  (params (Weapon :type "/Game/Data/E_Weapon Enum" :default "NewEnumerator0") (Equipment :type "/Game/Data/E_Equipment Enum" :default "NewEnumerator0") (WeaponState :type "/Game/Data/F_WeaponState Structure"))
  (bind _playercontroller (`self.PlayerController`))
  (`/Engine/EditorBlueprintResources/StandardMacros.IsValid` (select `/Game/Data/E_Equipment` Equipment :`NewEnumerator1` (`self.Weapon_Primary`) :`NewEnumerator2` (`self.Weapon_Secondary`) :!type "Object Object Reference")
    (:`Is Valid`
      (`self.SERVER_DropEquipment` Equipment))
    (:`Is Not Valid`
      _))
  (bind _returnvalue (`|SpawnActorFromClass` (`/Game/BlueprintLibraries/Game.GetWeaponClass` Weapon) (`self.GetTransform`) "AlwaysSpawn" "OverrideRootScale" _playercontroller (`/Game/Blueprints/BP_BaseGamemode.GetWeaponData` (`self.Base Gamemode`) Weapon) (`local.WeaponState`) self _playercontroller null))
  (switch `/Game/Data/E_Equipment` Equipment
    (:`NewEnumerator1`
      (set `self.Weapon_Primary` _returnvalue))
    (:`NewEnumerator2`
      (set `self.Weapon_Secondary` _returnvalue))))

(fn `PrintDebugInfo`
  (bind _kills (`self.GetKills`))
  (bind _assists (`self.GetAssists`))
  (bind _deaths (`self.GetDeaths`))
  (`KismetSystemLibrary.PrintString` (`KismetStringLibrary.Concat_StrStr` (`KismetSystemLibrary.GetDisplayName` self) ": " (`KismetStringLibrary.Concat_StrStr` (`KismetStringLibrary.Conv_IntToString` _kills) "/" (`KismetStringLibrary.Conv_IntToString` _assists) "/" (`KismetStringLibrary.Conv_IntToString` _deaths))) true true (`KismetMathLibrary.SelectColor` (struct :`G` 1.0 :`B` 0.161746 :`A` 1.0) (struct :`R` 1.0 :`G` 0.438138 :`A` 1.0) (`KismetSystemLibrary.IsServer`)) 0.0))

(fn `ReceiveDamage`
  (params (Instigator :type "Actor Object Reference") (DamageData :type "/Game/Data/F_DamageData Structure (by ref)"))
  (locals (TEMP_AreEnemies :type Boolean))
  (if (not (`self.IsDead`))
    (bind _team (`self.GetTeam`))
    (bind _team_2 (message `/Game/BlueprintInterfaces/BI_Game.GetTeam` Instigator))
    (bind _output_get (set `local.TEMP_AreEnemies` (`|EnumInequality` _team_2 _team)))
    (if (or _output_get (`/Game/BlueprintLibraries/Match.FriendlyFire` (`/Game/Blueprints/BP_BaseGamemode.GetMatchData` (`self.Base Gamemode`))))
      (bind _output_get_2 (set `self.Health` (- (`self.Health`) (`.Damage_2_23CE6C9F40CE3CE84C47479B407D4E01` (break `/Game/Data/F_DamageData` DamageData)))))
      (`self.CLIENT_Updatehealth` _output_get_2)
      (`|ExecutionSequence`
        (:`then_0`
          (if (and (`local.TEMP_AreEnemies`) (!= (`local.Instigator`) (`self.KillingInstigator`)))
            (`/Engine/EditorBlueprintResources/StandardMacros.IsValid` (`self.KillingInstigator`)
              (:`Is Valid`
                (set `self.AssistingInstigator` (`self.KillingInstigator`))
                (set `self.KillingInstigator` (`local.Instigator`)))
              (:`Is Not Valid`
                (set `self.KillingInstigator` (`local.Instigator`))))))
        (:`then_1`
          (if (<= (`self.Health`) 0.0)
            (set `self.IsDead` true)
            (`|ExecutionSequence`
              (:`then_0`
                (`|ExecutionSequence`
                  (:`then_0`
                    (if (`local.TEMP_AreEnemies`)
                      (message `/Game/BlueprintInterfaces/BI_Game.AddKill` (`local.Instigator`))
                      (`/Engine/EditorBlueprintResources/StandardMacros.IsValid` (`self.AssistingInstigator`)
                        (:`Is Valid`
                          (message `/Game/BlueprintInterfaces/BI_Game.AddAssist` (`self.AssistingInstigator`))))
                      (else
                        (`/Engine/EditorBlueprintResources/StandardMacros.IsValid` (`self.KillingInstigator`)
                          (:`Is Valid`
                            (message `/Game/BlueprintInterfaces/BI_Game.AddKill` (`self.KillingInstigator`))
                            (`/Engine/EditorBlueprintResources/StandardMacros.IsValid` (`self.AssistingInstigator`)
                              (:`Is Valid`
                                (message `/Game/BlueprintInterfaces/BI_Game.AddAssist` (`self.AssistingInstigator`)))))))))))
              (:`then_1`
                (`self.NETALL_OnDeath`)
                (`self.AddDeath` (`self.PlayerController`) (`local.Instigator`))
                (`/Game/Blueprints/BP_BaseGamemode.Remove Character` (`self.Base Gamemode`) (`self.PlayerController`))))
            (else
              (`self.SERVER_StartHealthRegen`))))))))

(fn `RemovePickup`
  (params (Pickup :type "/Game/Blueprints/BP_BasePickup Object Reference"))
  (`KismetArrayLibrary.Array_RemoveItem` (`self.Pickups`) Pickup))

(fn `SetActionState`
  (params (NewState :type "/Game/Data/E_ActionState Enum" :default "NewEnumerator0") (IsLocalPlayer :type Boolean))
  (returns (State :type "/Game/Data/E_ActionState Enum"))
  (`|ExecutionSequence`
    (:`then_0`
      (`self.UpdateAction` (`self.ActionState`) false (`local.IsLocalPlayer`))
      (`self.UpdateAction` (`local.NewState`) true (`local.IsLocalPlayer`))
      (set `self.ActionState` (`local.NewState`)))
    (:`then_1`
      (if (`local.IsLocalPlayer`)
        (`self.SERVER_SetActionState` (`local.NewState`))
        (return (`local.NewState`))
        (else
          (return (`local.NewState`)))))))

(fn `SetCameraLagValues`
  (params (`Lag Speed` :type "Float (double-precision)") (`Rotation Lag Speed` :type "Float (double-precision)"))
  (set `SpringArmComponent.CameraLagSpeed` `Lag Speed` (`self.CameraArm`))
  (set `SpringArmComponent.CameraRotationLagSpeed` (`local.Rotation Lag Speed`) (`self.CameraArm`)))

(fn `SetCurrentPickup`
  (params (Pickup :type "/Game/Blueprints/BP_BasePickup Object Reference"))
  (bind _wbp_pickup (`/Game/UserInterface/Gameplay/WBP_PlayerHUD.WBP_Pickup` (`/Game/Blueprints/BP_BasePlayerController.GetPlayerHUD` (`self.PlayerController`))))
  (bind _output_get (set `self.CurrentPickup` Pickup))
  (`/Engine/EditorBlueprintResources/StandardMacros.IsValid` _output_get
    (:`Is Valid`
      (bind _name (`/Game/UserInterface/Gameplay/Components/WBP_Pickup.GetPickupDisplayName` _wbp_pickup))
      (`/Game/UserInterface/Gameplay/Components/WBP_Pickup.UpdatePickup` _wbp_pickup _name true))
    (:`Is Not Valid`
      (`/Game/UserInterface/Gameplay/Components/WBP_Pickup.UpdatePickup` _wbp_pickup "" false))))

(fn `SetIsAiming`
  (params (IsAiming :type Boolean) (IsLocalPlayer :type Boolean))
  (bind _tl_aiming (`self.TL_Aiming`))
  (bind _output_get (set `self.bUseControllerRotationYaw` IsAiming))
  (set `CharacterMovementComponent.bOrientRotationToMovement` (not _output_get) (`self.CharacterMovement`))
  (`|ExecutionSequence`
    (:`then_0`
      (if (`local.IsAiming`)
        (set `CharacterMovementComponent.MaxWalkSpeed` (`self.PlayerSpeed_Aiming`) (`self.CharacterMovement`))))
    (:`then_1`
      (if (`local.IsLocalPlayer`)
        (if (`local.IsAiming`)
          (`TimelineComponent.Play` _tl_aiming)
          (`self.SetCameraLagValues` 30.0)
          (else
            (`TimelineComponent.Reverse` _tl_aiming)))))))

(fn `SetIsWalking`
  (params (IsWalking :type Boolean) (IsLocalPlayer :type Boolean))
  (if IsWalking
    (set `CharacterMovementComponent.MaxWalkSpeed` (`self.PlayerSpeed_Walking`) (`self.CharacterMovement`))
    (if (`local.IsLocalPlayer`)
      (`self.SetCameraLagValues` 20.0 20.0))))

(fn `Setup_Local`
  (set `self.PlayerController` (`/Game/BlueprintLibraries/Game.GetBasePlayerController`))
  (`self.StartPickupTimer`)
  (`ActorComponent.Activate` (`self.AUDIO_Heartbeat`) false))

(fn `Setup_NotLocal`
  (bind _team (`self.GetTeam`))
  (bind _team_2 (message `/Game/BlueprintInterfaces/BI_Game.GetTeam` (`GameplayStatics.GetPlayerController` 0)))
  (`self.CreatePlayerTag` (`/Game/BlueprintLibraries/Game.GetEntityColor` _team_2 _team)))

(fn `Tick_Client`
  (if (`self.IsLocallyControlled`)
    _))

(fn `UpdateAction`
  (params (Action :type "/Game/Data/E_ActionState Enum" :default "NewEnumerator0") (NewValue :type Boolean) (IsLocalPlayer :type Boolean))
  (switch `/Game/Data/E_ActionState` Action
    (:`NewEnumerator1`
      (`self.SetIsWalking` (`local.NewValue`) (`local.IsLocalPlayer`)))
    (:`NewEnumerator2`
      (`self.SetIsAiming` (`local.NewValue`) (`local.IsLocalPlayer`)))))

(fn `UpdateHealthFeedback`
  (params (HealthPercentage :type "Float (double-precision)"))
  (bind _audio_heartbeat (`self.AUDIO_Heartbeat`))
  (bind _returnvalue (- 1.0 (`local.HealthPercentage`)))
  (setmembers `PostProcessSettings` :`StructRef` (`CameraComponent.PostProcessSettings` (`self.PlayerCamera`)) :`ColorSaturation` (`KismetMathLibrary.MakeVector4` HealthPercentage HealthPercentage HealthPercentage HealthPercentage))
  (`AudioComponent.SetVolumeMultiplier` _audio_heartbeat _returnvalue)
  (`AudioComponent.SetPitchMultiplier` _audio_heartbeat (+ _returnvalue 0.8)))

(fn `UserConstructionScript`)