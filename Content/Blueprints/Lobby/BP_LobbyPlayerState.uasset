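; Lobby player state that holds a player's team selection.
; A client event steps to the next team, resetting to the first enum entry past the team count, then requests the change from the server.
; The server stores the team and relays it through a NETALL event, which fires OnTeamChanged.
; GetTeam returns the real value, while stat, name, focus location and gamemode getters are placeholders returning defaults.
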(event `CLIENT_OffsetTeam`
  (params (NumTeams :type Integer))
  (bind _returnvalue (+ (`KismetMathLibrary.Conv_ByteToInt` (`self.Team`)) 1))
  (if (> _returnvalue NumTeams)
    (`self.SERVER_SetTeam` "NewEnumerator0")
    (else
      (`self.SERVER_SetTeam` (cast `/Game/Data/E_Team` (`KismetMathLibrary.Conv_IntToByte` _returnvalue))))))

(event `SERVER_SetTeam`
  (params (Team :type "/Game/Data/E_Team Enum" :default "NewEnumerator0"))
  (bind _output_get (set `self.Team` Team))
  (`self.NETALL_SetTeam` _output_get))

(event `NETALL_SetTeam`
  (params (Team :type "/Game/Data/E_Team Enum" :default "NewEnumerator0"))
  (bind _output_get (set `self.Team` Team))
  (`self.OnTeamChanged` _output_get))

(fn `GetAssists`
  (returns (Assists :type Integer))
  (return 0))

(fn `GetDeaths`
  (returns (Deaths :type Integer))
  (return 0))

(fn `GetEntityName`
  (returns (Name :type Text))
  (return ""))

(fn `GetFocusLocation`
  (returns (Location :type "Vector Structure"))
  (return (0.0 0.0 0.0)))

(fn `GetGamemode`
  (returns (Gamemode :type "/Game/Data/E_Gamemode Enum"))
  (return "NewEnumerator0"))

(fn `GetKills`
  (returns (Kills :type Integer))
  (return 0))

(fn `GetScore`
  (returns (Score :type Integer))
  (return 0))

(fn `GetTeam`
  (returns (Team :type "/Game/Data/E_Team Enum"))
  (return (`self.Team`)))

(fn `UserConstructionScript`)