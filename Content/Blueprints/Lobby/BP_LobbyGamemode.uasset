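; Lobby game mode that manages a multiplayer session's players, server chat notices, map vote and launch into the match.
; On begin play it writes gamemode and server name to session settings and loads gamemode and map data tables.
; Voting offers two random maps from the gamemode's pool, breaking ties randomly, then a countdown runs servertravel with map and mode.
; Player controller client events keep each lobby UI in sync.
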(event `self.ReceiveBeginPlay`
  (bind _game_instance (`self.Game Instance`))
  ;[0 0 0] Begin Play
  (set `self.Game Instance` (`/Game/BlueprintLibraries/Game.GetGameInstance`))
  (bind (_numconnections _numprivateconnections _bislan _bisdedicated _ballowinvites _ballowjoininprogress _bisanticheatenabled _builduniqueid _extrasettings) (`AdvancedSessionsLibrary.GetSessionSettings`)
    (:`OnSuccess`
      (set `self.Settings` _extrasettings)
      (`self.SetGamemode` (`/Game/Blueprints/BP_GameInstance.UI_CreationGamemode` _game_instance))
      (`self.SetServerName` (`KismetTextLibrary.Conv_TextToString` (`/Game/Blueprints/BP_GameInstance.UI_CreationName` _game_instance)))
      (`self.FetchGamemodeData`)
      (`self.FetchMapData`)
      (`self.UpdateSessionSettings`))))

(event `self.HandleStartingNewPlayer`
  (params (NewPlayer :type "PlayerController Object Reference"))
  ;[0 0 0] Starting new player
  (bind _asbp_lobby_player_controller (cast `/Game/Blueprints/Lobby/BP_LobbyPlayerController` NewPlayer))
  (`KismetArrayLibrary.Array_Add` (`self.Players`) _asbp_lobby_player_controller)
  (`/Game/Blueprints/Lobby/BP_LobbyPlayerController.CLIENT_Setup` _asbp_lobby_player_controller)
  (`/Game/Blueprints/Lobby/BP_LobbyPlayerController.CLIENT_ChangeGamemode` _asbp_lobby_player_controller (`self.Gamemode`))
  (bind _asbp_lobby_player_state (cast `/Game/Blueprints/Lobby/BP_LobbyPlayerState` (`Controller.PlayerState` _asbp_lobby_player_controller)))
  (`KismetArrayLibrary.Array_Add` (`self.PlayerStates`) _asbp_lobby_player_state)
  (`KismetSystemLibrary.Delay` 7.0)
  (`/Game/Blueprints/Lobby/BP_LobbyPlayerController.CLIENT_CreateLobby` _asbp_lobby_player_controller)
  (`self.UpdateClientsLobby` (`self.PlayerStates`)))

(event `self.K2_OnLogout`
  (params (ExitingController :type "Controller Object Reference"))
  ;[0 0 0] Log out player
  (bind _asbp_lobby_player_controller (cast `/Game/Blueprints/Lobby/BP_LobbyPlayerController` ExitingController))
  (if (`KismetArrayLibrary.Array_Contains` (`self.Players`) _asbp_lobby_player_controller)
    (bind _returnvalue (`KismetArrayLibrary.Array_RemoveItem` (`self.Players`) _asbp_lobby_player_controller))
    (if _returnvalue
      (bind _asbp_lobby_player_state (cast `/Game/Blueprints/Lobby/BP_LobbyPlayerState` (`Controller.PlayerState` _asbp_lobby_player_controller)))
      (if (`KismetArrayLibrary.Array_Contains` (`self.PlayerStates`) _asbp_lobby_player_state)
        (bind _returnvalue_2 (`KismetArrayLibrary.Array_RemoveItem` (`self.PlayerStates`) _asbp_lobby_player_state))
        (if _returnvalue_2
          (`self.SendChatMessage` (make `/Game/Data/F_ChatMessage` "SERVER" "A player has left the game!"))
          (`KismetSystemLibrary.Delay` 0.4)
          (`self.UpdateClientsLobby` (`self.PlayerStates`)))))))

(event `UpdateSessionSettings`
  ;[0 0 0] Updating session settings
  (bind (_numconnections _numprivateconnections _bislan _bisdedicated _ballowinvites _ballowjoininprogress _bisanticheatenabled) (`AdvancedSessionsLibrary.GetSessionSettings`)
    (:`OnSuccess`
      (`UpdateSessionCallbackProxyAdvanced.UpdateSession` (`self.Settings`) _numconnections _numprivateconnections _bislan _bisdedicated _ballowinvites _ballowjoininprogress _bisanticheatenabled))))

(event `Start Voting Timer`
  (params (Time :type Integer))
  ;[0 0 0] Timers for votings and starting the game
  (set `self.VotingTime` Time)
  (bind _returnvalue (`KismetSystemLibrary.K2_SetTimerDelegate` (delegate `EVENT_OnVotingTimeUpdate`) 1.0 true))
  (set `self.Timer_Voting` _returnvalue))

(event `EVENT_OnVotingTimeUpdate`
  ;[0 0 0] Timers for votings and starting the game
  (bind _result (`/Engine/EditorBlueprintResources/StandardMacros.DecrementInt` (`self.VotingTime`))
    (:`  `
      (if (<= _result 0)
        (`KismetSystemLibrary.K2_ClearAndInvalidateTimerHandle` (`self.Timer_Voting`))
        (`self.FinishVoting`)))))

(event `Start Starting Timer`
  (params (Time :type Integer))
  ;[0 0 0] Timers for votings and starting the game
  (set `self.StartingTime` Time)
  (bind _returnvalue (`KismetSystemLibrary.K2_SetTimerDelegate` (delegate `EVENT_OnStartTimeUpdate`) 1.0 true))
  (set `self.Timer_Starting` _returnvalue))

(event `EVENT_OnStartTimeUpdate`
  ;[0 0 0] Timers for votings and starting the game
  (bind _result (`/Engine/EditorBlueprintResources/StandardMacros.DecrementInt` (`self.StartingTime`))
    (:`  `
      (if (<= _result 0)
        (`KismetSystemLibrary.K2_ClearAndInvalidateTimerHandle` (`self.Timer_Starting`))
        (`self.CloseClientsLobby`)
        (`KismetSystemLibrary.Delay` 1.0)
        (`self.StartGame`)))))

(event `self.K2_PostLogin`
  (params (NewPlayer :type "PlayerController Object Reference"))
  (`self.SendChatMessage` (make `/Game/Data/F_ChatMessage` "SERVER" "A new player is joining the game!")))

(fn `CancelGameStartup`
  (`KismetSystemLibrary.K2_ClearAndInvalidateTimerHandle` (`self.Timer_Voting`))
  (`KismetSystemLibrary.K2_ClearAndInvalidateTimerHandle` (`self.Timer_Starting`))
  (for _array_element (`self.Players`)
    (`/Game/Blueprints/Lobby/BP_LobbyPlayerController.CLIENT_CancelGameStartup` _array_element)))

(fn `CloseClientsLobby`
  (for _array_element (`self.Players`)
    (`/Game/Blueprints/Lobby/BP_LobbyPlayerController.CLIENT_CloseLobby` _array_element)))

(fn `FetchGamemodeData`
  (bind _outrownames (`DataTableFunctionLibrary.GetDataTableRowNames` "/Game/Data/DT_Gamemodes.DT_Gamemodes"))
  (for _array_element _outrownames
    (bind _returnvalue (`|GetDataTableRow` "/Game/Data/DT_Gamemodes.DT_Gamemodes" _array_element)
      (:`then`
        (`KismetArrayLibrary.Array_Add` (`self.GamemodeData`) _returnvalue)))))

(fn `FetchMapData`
  (bind _outrownames (`DataTableFunctionLibrary.GetDataTableRowNames` "/Game/Data/DT_Maps.DT_Maps"))
  (for _array_element _outrownames
    (bind _returnvalue (`|GetDataTableRow` "/Game/Data/DT_Maps.DT_Maps" _array_element)
      (:`then`
        (`KismetArrayLibrary.Array_Add` (`self.MapData`) _returnvalue)))))

(fn `FindFinalMap`
  (returns (MapOption_1 :type "/Game/Data/F_Map Structure"))
  (if (> (`self.VoteRatio`) 0)
    (return (`self.MapOption_1`))
    (elif (< (`self.VoteRatio`) 0)
      (return (`self.MapOption_2`))
      (elif (`KismetMathLibrary.RandomBool`)
        (return (`self.MapOption_1`))
        (else
          (return (`self.MapOption_2`)))))))

(fn `FindMapPool`
  (`KismetArrayLibrary.Array_Clear` (`self.MapPool`))
  (for _array_element (`self.MapData`)
    (for _array_element_2 (`.Gamemode_Maps_22_38D34ED14B8AE1C3361A2AA6B51CE615` (break `/Game/Data/F_Gamemode` (`|GetArrayItem` (`self.GamemodeData`) (`KismetMathLibrary.Conv_ByteToInt` (`self.Gamemode`)))))
      (bind _map_name (break `/Game/Data/F_Map` _array_element))
      (if (== _array_element_2 _map_name)
        (`KismetArrayLibrary.Array_Add` (`self.MapPool`) _array_element)
        (`KismetSystemLibrary.PrintString` (`KismetTextLibrary.Conv_TextToString` _map_name))))))

(fn `FinishVoting`
  (set `self.FinalMap` (`self.FindFinalMap`))
  (for _array_element (`self.Players`)
    (`/Game/Blueprints/Lobby/BP_LobbyPlayerController.CLIENT_SwitchToFinalScreen` _array_element (`self.FinalMap`) 8))
  (`self.Start Starting Timer` 8))

(fn `GetGamemodeCommand`
  (returns (Gamemode :type String))
  (return (`|GetEnumeratorNameAsString` (`self.Gamemode`))))

(fn `GetGamemodeData`
  (returns (Data :type "/Game/Data/F_Gamemode Structure (by ref)"))
  (return (`|GetArrayItem` (`self.GamemodeData`) (`KismetMathLibrary.Conv_ByteToInt` (`self.Gamemode`)))))

(fn `GetMapNameCommand`
  (returns (MapName :type String))
  (return (`KismetStringLibrary.Conv_NameToString` (`.Map_UnrealName_12_F446A849485AE5A6937F979813737E3E` (break `/Game/Data/F_Map` (`self.FinalMap`))))))

(fn `GetStartCommand`
  (returns (Command :type String))
  (return (`KismetStringLibrary.Concat_StrStr` "servertravel " (`self.GetMapNameCommand`) "?game=" (`self.GetGamemodeCommand`))))

(fn `RandomizeMapOptions`
  (locals (TEMP_MapPool :type "Array of /Game/Data/F_Map Structure") (TEMP_Index :type Integer :default 0))
  (bind _output_get (set `local.TEMP_MapPool` (`self.MapPool`)))
  (set `local.TEMP_Index` (`.OutIndex` (`KismetArrayLibrary.Array_Random` _output_get)))
  (set `self.MapOption_1` (`|GetArrayItem` (`local.TEMP_MapPool`) (`local.TEMP_Index`)))
  (`KismetArrayLibrary.Array_Remove` (`local.TEMP_MapPool`) (`local.TEMP_Index`))
  (set `self.MapOption_2` (`KismetArrayLibrary.Array_Random` (`local.TEMP_MapPool`))))

(fn `SendChatMessage`
  (params (`Chat Message` :type "/Game/Data/F_ChatMessage Structure"))
  (for _array_element (`self.Players`)
    (`/Game/Blueprints/Lobby/BP_LobbyPlayerController.CLIENT_ReceiveChatMessage` _array_element (`local.Chat Message`))))

(fn `SetGamemode`
  (params (Gamemode :type "/Game/Data/E_Gamemode Enum" :default "NewEnumerator0"))
  (set `self.Gamemode` Gamemode)
  (bind _modifiedsettingsarray (`AdvancedSessionsLibrary.AddOrModifyExtraSettings` (`self.Settings`) (`|MakeArray` (`AdvancedSessionsLibrary.MakeLiteralSessionPropertyByte` "GAMEMODE" (`self.Gamemode`)))))
  (set `self.Settings` _modifiedsettingsarray)
  (for _array_element (`self.Players`)
    (`/Game/Blueprints/Lobby/BP_LobbyPlayerController.CLIENT_ChangeGamemode` _array_element (`self.Gamemode`))))

(fn `SetServerName`
  (params (Name :type String))
  (bind _modifiedsettingsarray (`AdvancedSessionsLibrary.AddOrModifyExtraSettings` (`self.Settings`) (`|MakeArray` (`AdvancedSessionsLibrary.MakeLiteralSessionPropertyString` "NAME" (`local.Name`)))))
  (set `self.Settings` _modifiedsettingsarray))

(fn `StartGame`
  (`KismetSystemLibrary.PrintString` "Game is starting...")
  (`KismetSystemLibrary.ExecuteConsoleCommand` (`self.GetStartCommand`) (`GameplayStatics.GetPlayerController` 0)))

(fn `StartVoting`
  (`self.FindMapPool`)
  (`self.RandomizeMapOptions`)
  (for _array_element (`self.Players`)
    (`/Game/Blueprints/Lobby/BP_LobbyPlayerController.CLIENT_SwitchToVoting` _array_element (`self.MapOption_1`) (`self.MapOption_2`) 10))
  (`self.Start Voting Timer` 10))

(fn `Update Map Votes`
  (locals (Count_Map1 :type Integer) (Count_Map2 :type Integer))
  (for _array_element (`self.Players`)
    (switch `/Game/Data/E_MapVote` (`/Game/Blueprints/Lobby/BP_LobbyPlayerController.GetPlayerVote` _array_element)
      (:`NewEnumerator1`
        (`/Engine/EditorBlueprintResources/StandardMacros.IncrementInt` (`local.Count_Map1`)))
      (:`NewEnumerator2`
        (`/Engine/EditorBlueprintResources/StandardMacros.IncrementInt` (`local.Count_Map2`)))))
  (for _array_element_2 (`self.Players`)
    (`/Game/Blueprints/Lobby/BP_LobbyPlayerController.CLIENT_UpdateVotes` _array_element_2 (`local.Count_Map1`) (`local.Count_Map2`)))
  (set `self.VoteRatio` (- (`local.Count_Map1`) (`local.Count_Map2`))))

(fn `UpdateClientsLobby`
  (params (PlayerStates :type "Array of /Game/Blueprints/Lobby/BP_LobbyPlayerState Object Reference"))
  (for _array_element (`self.Players`)
    (`/Game/Blueprints/Lobby/BP_LobbyPlayerController.CLIENT_UpdateLobby` _array_element PlayerStates)))

(fn `UserConstructionScript`)