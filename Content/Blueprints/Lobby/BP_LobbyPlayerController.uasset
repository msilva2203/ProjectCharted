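; Lobby player controller that runs each client's lobby menu, from player list and team switching to map voting and the starting countdown.
; Client events create the menu and transition widgets, switch screens and run one-second countdown and list-refresh timers, with gamemode rules read from DT_Gamemodes.
; Map votes and chat messages go through server events to the lobby gamemode.
; Replication of LobbyPlayers creates the lobby if missing and refreshes the list after a short delay.
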(event `self.ReceiveBeginPlay`
  (if (`self.IsLocalPlayerController`)
    _))

(event `OnLobbyUpdateReady`
  (if (`self.IsLocalPlayerController`)
    (`KismetSystemLibrary.Delay` 0.5)
    (`|ExecutionSequence`
      (:`then_0`
        (if (not (`KismetSystemLibrary.IsValid` (`self.Lobby`)))
          (`self.CLIENT_CreateLobby`)))
      (:`then_1`
        (`self.CLIENT_UpdateLobby` (`self.Lobby Players`))
        (`self.UpdateCanSwitchTeam`)))))

(event `Start Voting Timer`
  (params (Time :type Integer))
  ;[0 0 0] Voting timer
  (set `self.VotingTime` Time)
  (`/Game/UserInterface/Menus/SubMenus/WBP_Lobby.UpdateVotingTime` (`/Game/UserInterface/Menus/WBP_LobbyMenu.WBP_Lobby` (`self.Lobby`)) (`self.VotingTime`))
  (bind _returnvalue (`KismetSystemLibrary.K2_SetTimerDelegate` (delegate `EVENT_VotingTimeUpdate`) 1.0 true))
  (set `self.Timer_Voting` _returnvalue))

(event `EVENT_VotingTimeUpdate`
  ;[0 0 0] Voting timer
  (set `self.VotingTime` (`KismetMathLibrary.Clamp` (- (`self.VotingTime`) 1) 0 100))
  (`/Game/UserInterface/Menus/SubMenus/WBP_Lobby.UpdateVotingTime` (`/Game/UserInterface/Menus/WBP_LobbyMenu.WBP_Lobby` (`self.Lobby`)) (`self.VotingTime`)))

(event `Start Starting Timer`
  (params (Time :type Integer))
  ;[0 0 0] Start Timer
  (bind _output_get (set `self.StartingTime` Time))
  (`/Game/UserInterface/Menus/SubMenus/WBP_Lobby.UpdateStartingTime` (`/Game/UserInterface/Menus/WBP_LobbyMenu.WBP_Lobby` (`self.Lobby`)) _output_get)
  (bind _returnvalue (`KismetSystemLibrary.K2_SetTimerDelegate` (delegate `EVENT_StartTimeUpdate`) 1.0 true))
  (set `self.Timer_Starting` _returnvalue))

(event `EVENT_StartTimeUpdate`
  ;[0 0 0] Start Timer
  (set `self.StartingTime` (`KismetMathLibrary.Clamp` (- (`self.StartingTime`) 1) 0 100))
  (`/Game/UserInterface/Menus/SubMenus/WBP_Lobby.UpdateStartingTime` (`/Game/UserInterface/Menus/WBP_LobbyMenu.WBP_Lobby` (`self.Lobby`)) (`self.StartingTime`)))

(event `Start Refresh Timer`
  ;[0 0 0] Player list refreshing
  (bind _returnvalue (`KismetSystemLibrary.K2_SetTimerDelegate` (delegate `EVENT_OnRefresh`) 1.0 true))
  (set `self.Timer_Refresh` _returnvalue))

(event `EVENT_OnRefresh`
  ;[0 0 0] Player list refreshing
  (`/Game/UserInterface/Menus/SubMenus/WBP_LobbyPlayerList.Refresh` (`/Game/UserInterface/Menus/WBP_LobbyMenu.EBP_LobbyPlayerList` (`self.Lobby`))))

(event `self.ReceiveEndPlay`
  (params (EndPlayReason :type "EEndPlayReason Enum" :default "Destroyed"))
  (if (`self.IsLocalController`)
    (`Widget.RemoveFromParent` (`self.Lobby`))
    (`Widget.RemoveFromParent` (`self.TransitionWidget`))))

(event `CLIENT_Setup`
  (`self.FetchGamemodeData`)
  (`self.CreateTransitionWidget`))

(event `CLIENT_ChangeGamemode`
  (params (NewGamemode :type "/Game/Data/E_Gamemode Enum" :default "NewEnumerator0"))
  (set `self.Gamemode` NewGamemode)
  (`self.UpdateGamemodeName`)
  (`self.UpdateMaxPlayers`)
  (`self.UpdateCanSwitchTeam`))

(event `CLIENT_CreateLobby`
  (bind _transitionwidget (`self.GetTransitionWidget`))
  (`self.ShowLobbyMenu`)
  (`self.UpdateGamemodeName`)
  (`self.UpdateMaxPlayers`)
  (if (`/Game/UserInterface/Menus/SubMenus/WBP_Transition.IsFull` _transitionwidget)
    (`/Game/UserInterface/Menus/SubMenus/WBP_Transition.PlayTransition` _transitionwidget (delegate `EVENT`) "Reverse" 2.0)
    (`Widget.SetVisibility` (`self.GetTransitionWidget`) "HitTestInvisible")))

(event `EVENT`)

(event `CLIENT_CloseLobby`
  (`/Game/UserInterface/Menus/SubMenus/WBP_Transition.PlayTransition` (`self.GetTransitionWidget`) (delegate `EVENT 1`) "Forward" 3.0)
  (`Widget.SetVisibility` (`self.GetTransitionWidget`) "Visible"))

(event `EVENT 1`)

(event `CLIENT_UpdateLobby`
  (params (PlayerStates :type "Array of /Game/Blueprints/Lobby/BP_LobbyPlayerState Object Reference"))
  (`/Game/UserInterface/Menus/SubMenus/WBP_LobbyPlayerList.PopulatePlayers` (`/Game/UserInterface/Menus/WBP_LobbyMenu.EBP_LobbyPlayerList` (`self.Lobby`)) PlayerStates)
  (`self.Start Refresh Timer`)
  (`self.UpdateMaxPlayers`))

(event `CLIENT_SwitchToVoting`
  (params (`Map 1` :type "/Game/Data/F_Map Structure") (`Map 2` :type "/Game/Data/F_Map Structure") (Time :type Integer))
  (bind _wbp_lobby (`/Game/UserInterface/Menus/WBP_LobbyMenu.WBP_Lobby` (`self.Lobby`)))
  (`/Game/UserInterface/Menus/SubMenus/WBP_Lobby.UpdateMapDisplays` _wbp_lobby `Map 1` `Map 2`)
  (`/Game/UserInterface/Menus/SubMenus/WBP_Lobby.SwitchToMapVoting` _wbp_lobby)
  (`self.Start Voting Timer` Time)
  (`/Game/UserInterface/Menus/WBP_LobbyMenu.SetCanSwitchTeam` (`self.Lobby`) false))

(event `CLIENT_SwitchToFinalScreen`
  (params (MapData :type "/Game/Data/F_Map Structure") (Time :type Integer))
  (bind _wbp_lobby (`/Game/UserInterface/Menus/WBP_LobbyMenu.WBP_Lobby` (`self.Lobby`)))
  (`/Game/UserInterface/Menus/SubMenus/WBP_Lobby.UpdateFinalMap` _wbp_lobby MapData)
  (`/Game/UserInterface/Menus/SubMenus/WBP_Lobby.SwitchToFinalScreen` _wbp_lobby)
  (`self.Start Starting Timer` Time)
  (`KismetSystemLibrary.K2_ClearAndInvalidateTimerHandle` (`self.Timer_Voting`))
  (`/Game/UserInterface/Menus/WBP_LobbyMenu.SetCanSwitchTeam` (`self.Lobby`) false))

(event `CLIENT_CancelGameStartup`
  (`/Game/UserInterface/Menus/SubMenus/WBP_Lobby.SwitchToMainLobby` (`/Game/UserInterface/Menus/WBP_LobbyMenu.WBP_Lobby` (`self.Lobby`)))
  (`KismetSystemLibrary.K2_ClearAndInvalidateTimerHandle` (`self.Timer_Voting`))
  (`KismetSystemLibrary.K2_ClearAndInvalidateTimerHandle` (`self.Timer_Starting`))
  (`self.UpdatePlayerVote` "NewEnumerator0")
  (`self.UpdateCanSwitchTeam`)
  (`self.UpdateMaxPlayers`))

(event `SERVER_UpdatePlayerVote`
  (params (NewVote :type "/Game/Data/E_MapVote Enum" :default "NewEnumerator0"))
  (set `self.MapVote` NewVote)
  (`/Game/Blueprints/Lobby/BP_LobbyGamemode.Update Map Votes` (`/Game/BlueprintLibraries/Game.GetLobbyGamemode`)))

(event `CLIENT_UpdateVotes`
  (params (VoteCount_Map1 :type Integer) (VoteCount_Map2 :type Integer))
  (`/Game/UserInterface/Menus/SubMenus/WBP_Lobby.UpdateMapVotes` (`/Game/UserInterface/Menus/WBP_LobbyMenu.WBP_Lobby` (`self.Lobby`)) VoteCount_Map1 VoteCount_Map2))

(event `CLIENT_ReceiveChatMessage`
  (params (`Chat Message` :type "/Game/Data/F_ChatMessage Structure"))
  (bind _lobby (`self.Lobby`))
  (`/Engine/EditorBlueprintResources/StandardMacros.IsValid` _lobby
    (:`Is Valid`
      (`/Game/UserInterface/Components/WBP_ChatBox.AddChatMessage` (`/Game/UserInterface/Menus/WBP_LobbyMenu.WBP_ChatBox` _lobby) `Chat Message`))))

(event `CLIENT_SendChatMessage`
  (params (Message :type Text))
  (`self.SERVER_SendChatMessage` Message))

(event `SERVER_SendChatMessage`
  (params (Message :type Text))
  (`/Game/Blueprints/Lobby/BP_LobbyGamemode.SendChatMessage` (`/Game/BlueprintLibraries/Game.GetLobbyGamemode`) (make `/Game/Data/F_ChatMessage` (`KismetTextLibrary.Conv_StringToText` (`PlayerState.GetPlayerName` (`self.PlayerState`))) Message)))

(event `CLIENT_SetCanSwitchTeams`
  (params (CanSwitch :type Boolean))
  (`/Game/UserInterface/Menus/WBP_LobbyMenu.SetCanSwitchTeam` (`self.Lobby`) CanSwitch))

(event `CLIENT_HideUnfoundPlayers`
  (`/Game/UserInterface/Menus/SubMenus/WBP_LobbyPlayerList.HideUnfoundPlayers` (`/Game/UserInterface/Menus/WBP_LobbyMenu.EBP_LobbyPlayerList` (`self.Lobby`))))

(fn `CreateTransitionWidget`
  (bind _returnvalue (`|CreateWidget` "/Game/UserInterface/Menus/SubMenus/WBP_Transition.WBP_Transition_C" self))
  (bind _output_get (set `self.TransitionWidget` _returnvalue))
  (`UserWidget.AddToViewport` _output_get 999)
  (`/Game/UserInterface/Menus/SubMenus/WBP_Transition.FillScreen` (`self.GetTransitionWidget`)))

(fn `FetchGamemodeData`
  (bind _outrownames (`DataTableFunctionLibrary.GetDataTableRowNames` "/Game/Data/DT_Gamemodes.DT_Gamemodes"))
  (for _array_element _outrownames
    (bind _returnvalue (`|GetDataTableRow` "/Game/Data/DT_Gamemodes.DT_Gamemodes" _array_element)
      (:`then`
        (`KismetArrayLibrary.Array_Add` (`self.GamemodeData`) _returnvalue)))))

(fn `GetPlayerVote`
  (returns (MapVote :type "/Game/Data/E_MapVote Enum"))
  (return (`self.MapVote`)))

(fn `GetTransitionWidget`
  (returns (TransitionWidget :type "/Game/UserInterface/Menus/SubMenus/WBP_Transition Object Reference"))
  (return (`self.TransitionWidget`)))

(fn `OffsetTeam`
  (bind _asbp_lobby_player_state (cast `/Game/Blueprints/Lobby/BP_LobbyPlayerState` (`self.PlayerState`)))
  (`/Game/Blueprints/Lobby/BP_LobbyPlayerState.CLIENT_OffsetTeam` _asbp_lobby_player_state (`.Gamemode_NumTeams_30_20DF246241B152D3C016F49BCCCC9E4A` (break `/Game/Data/F_Gamemode` (`|GetArrayItem` (`self.GamemodeData`) (`KismetMathLibrary.Conv_ByteToInt` (`self.Gamemode`)))))))

(fn `OnRep_Lobby Players`
  (`self.OnLobbyUpdateReady`))

(fn `SetLobbyPlayers`
  (params (LobbyPlayers :type "Array of /Game/Blueprints/Lobby/BP_LobbyPlayerState Object Reference"))
  (set `self.Lobby Players` LobbyPlayers))

(fn `ShowLobbyMenu`
  (bind _returnvalue (`|CreateWidget` "/Game/UserInterface/Menus/WBP_LobbyMenu.WBP_LobbyMenu_C" (`GameplayStatics.GetPlayerController` 0)))
  (bind _output_get (set `self.Lobby` _returnvalue))
  (`UserWidget.AddToViewport` _output_get 0)
  (`WidgetBlueprintLibrary.SetInputMode_UIOnlyEx` self (`self.Lobby`))
  (set `self.bShowMouseCursor` true)
  (`Widget.SetFocus` (`self.Lobby`)))

(fn `UpdateCanSwitchTeam`
  (`/Game/UserInterface/Menus/WBP_LobbyMenu.SetCanSwitchTeam` (`self.Lobby`) (`.Gamemode_CanChooseTeam_29_5B8740634CE6BAC995262BAB60479B42` (break `/Game/Data/F_Gamemode` (`|GetArrayItem` (`self.GamemodeData`) (`KismetMathLibrary.Conv_ByteToInt` (`self.Gamemode`)))))))

(fn `UpdateGamemodeName`
  (`/Engine/EditorBlueprintResources/StandardMacros.IsValid` (`self.Lobby`)
    (:`Is Valid`
      (`/Game/UserInterface/Menus/SubMenus/WBP_Lobby.SetGamemodeName` (`/Game/UserInterface/Menus/WBP_LobbyMenu.WBP_Lobby` (`self.Lobby`)) (`.Gamemode_Name_3_B2026A494142BA9CEB0FFF961F0871EB` (break `/Game/Data/F_Gamemode` (`|GetArrayItem` (`self.GamemodeData`) (`KismetMathLibrary.Conv_ByteToInt` (`self.Gamemode`)))))))))

(fn `UpdateMaxPlayers`
  (bind _lobby (`self.Lobby`))
  (`/Engine/EditorBlueprintResources/StandardMacros.IsValid` _lobby
    (:`Is Valid`
      (`/Game/UserInterface/Menus/SubMenus/WBP_LobbyPlayerList.UpdateMaxPlayers` (`/Game/UserInterface/Menus/WBP_LobbyMenu.EBP_LobbyPlayerList` _lobby) (`.Gamemode_MaxPlayers_25_6B17F7314305E228953E1A9000C5F989` (break `/Game/Data/F_Gamemode` (`|GetArrayItem` (`self.GamemodeData`) (`KismetMathLibrary.Conv_ByteToInt` (`self.Gamemode`)))))))))

(fn `UpdatePlayerVote`
  (params (Vote :type "/Game/Data/E_MapVote Enum" :default "NewEnumerator0"))
  (if (`|EnumInequality` Vote (`self.MapVote`))
    (bind _output_get (set `self.MapVote` (`local.Vote`)))
    (`self.SERVER_UpdatePlayerVote` _output_get)))

(fn `UserConstructionScript`)