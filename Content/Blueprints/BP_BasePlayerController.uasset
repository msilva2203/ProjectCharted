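; Base player controller for multiplayer arena matches, handling each player's UI, scoring feedback, death, respawn and spectating.
; Server events update PlayerState stats and use client RPCs for sounds, money pickups, death camera and countdown.
; Respawns go through the gamemode, either on individual timers or in timed waves.
; Dead players cycle teammate or arena cameras; game HUD, scoreboard and feed functions are mostly stubs, apparently for child classes.
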(event `OnReady`
  (`KismetSystemLibrary.Delay` 1.0)
  (if (not (`self.Ready`))
    (`self.SERVER_OnReady`)
    (set `self.Ready` true)))

(event `self.ReceiveBeginPlay`
  (`|ExecutionSequence`
    (:`then_0`
      (if (`self.IsLocalController`)
        (bind _outactors (`GameplayStatics.GetAllActorsOfClass` "/Game/Blueprints/BP_ArenaCamera.BP_ArenaCamera_C"))
        (set `self.ArenaCameras` _outactors)))
    (:`then_1`
      (bind _asbp_base_player_state (cast `/Game/Blueprints/BP_BasePlayerState` (`self.PlayerState`)))
      (set `self.BasePlayerState` _asbp_base_player_state))
    (:`then_2`
      (if (`KismetSystemLibrary.IsServer`)
        (set `self.BaseGamemode` (`/Game/BlueprintLibraries/Game.GetBaseGamemode`))))))

(event `/Game/BlueprintInterfaces/BI_Game.AddKill`
  (params (KilledActor :type "Actor Object Reference"))
  (bind _location (message `/Game/BlueprintInterfaces/BI_Game.GetMoneyLocation` KilledActor))
  (`self.CLIENT_SpawnMoney` 100 "NewEnumerator1" _location)
  (`/Game/Blueprints/BP_BasePlayerState.OffsetKills` (`self.BasePlayerState`) 1)
  (`self.CLIENT_OnKill`)
  (`/Engine/EditorBlueprintResources/StandardMacros.IsValid` (`self.PlayerCharacter`)
    (:`Is Valid`
      (`/Game/BlueprintInterfaces/BI_Game.AddKill` (`self.PlayerCharacter`) KilledActor))))

(event `/Game/BlueprintInterfaces/BI_Game.AddAssist`
  (params (AssistedActor :type "Actor Object Reference"))
  (bind _location (message `/Game/BlueprintInterfaces/BI_Game.GetMoneyLocation` AssistedActor))
  (`self.CLIENT_SpawnMoney` 25 "NewEnumerator2" _location)
  (`/Game/Blueprints/BP_BasePlayerState.OffsetAssists` (`self.BasePlayerState`) 1)
  (`self.CLIENT_OnAssist`)
  (`/Engine/EditorBlueprintResources/StandardMacros.IsValid` (`self.PlayerCharacter`)
    (:`Is Valid`
      (`/Game/BlueprintInterfaces/BI_Game.AddAssist` (`self.PlayerCharacter`) AssistedActor))))

(event `/Game/BlueprintInterfaces/BI_Game.AddDeath`
  (params (Killer :type "Actor Object Reference"))
  (`self.OnDeath (OnServer)` Killer)
  (`/Game/Blueprints/BP_BasePlayerState.SetIsDead` (`self.BasePlayerState`) true))

(event `self.ReceivePossess`
  (params (PossessedPawn :type "Pawn Object Reference"))
  (bind _playercharacter (`self.PlayerCharacter`))
  (`self.CLIENT_OnPossess`)
  (`/Engine/EditorBlueprintResources/StandardMacros.IsValid` _playercharacter
    (:`Is Valid`
      (`self.K2_DestroyActor` _playercharacter))
    (:`Is Not Valid`
      _))
  (bind _asbp_base_character (cast `/Game/Blueprints/BP_BaseCharacter` PossessedPawn))
  (set `self.PlayerCharacter` _asbp_base_character))

(event `self.ReceiveUnPossess`
  (params (UnpossessedPawn :type "Pawn Object Reference"))
  (`self.CLIENT_OnUnpossess`))

(event `StartRespawnTimer`
  (params (Time :type Integer))
  (bind _wbp_respawnui (`/Game/UserInterface/Gameplay/WBP_PlayerHUD.WBP_RespawnUI` (`self.GetPlayerHUD`)))
  (set `self.RespawnTime` Time)
  (if (`self.IsLocalController`)
    (`/Game/UserInterface/Gameplay/Components/WBP_RespawnUI.SetVisible` _wbp_respawnui true)
    (`/Game/UserInterface/Gameplay/Components/WBP_RespawnUI.UpdateTime` _wbp_respawnui (`self.RespawnTime`)))
  (bind _returnvalue (`KismetSystemLibrary.K2_SetTimerDelegate` (delegate `EVENT_OnRespawnTimeUpdate`) 1.0 true))
  (set `self.Timer_Respawn` _returnvalue))

(event `EVENT_OnRespawnTimeUpdate`
  (`/Engine/EditorBlueprintResources/StandardMacros.DecrementInt` (`self.RespawnTime`)
    (:`  `
      (`|ExecutionSequence`
        (:`then_0`
          (if (`self.IsLocalController`)
            (if (> (`self.RespawnTime`) 0)
              (`/Game/UserInterface/Gameplay/Components/WBP_RespawnUI.UpdateTime` (`/Game/UserInterface/Gameplay/WBP_PlayerHUD.WBP_RespawnUI` (`self.GetPlayerHUD`)) (`self.RespawnTime`))
              (`GameplayStatics.PlaySound2D` "/Game/SFX/Gameplay/SC_MP_CLOCK.SC_MP_CLOCK" 1.0 1.0 0.0 null null)
              (else
                (`/Game/UserInterface/Gameplay/Components/WBP_RespawnUI.SetToRespawning` (`/Game/UserInterface/Gameplay/WBP_PlayerHUD.WBP_RespawnUI` (`self.GetPlayerHUD`)))
                (`GameplayStatics.PlaySound2D` "/Game/SFX/Gameplay/SC_MP_RESPAWN.SC_MP_RESPAWN" 1.0 1.0 0.0 null null)
                (`KismetSystemLibrary.K2_ClearAndInvalidateTimerHandle` (`self.Timer_Respawn`))))))))))

(event `StartServer_RespawnTimer`
  (params (RespawnTime :type Integer))
  (bind _returnvalue (`KismetSystemLibrary.K2_SetTimerDelegate` (delegate `EVENT_OnServerRespawn`) (`KismetMathLibrary.Conv_IntToDouble` RespawnTime)))
  (set `self.Timer_ServerRepsawn` _returnvalue))

(event `EVENT_OnServerRespawn`
  (`/Game/Blueprints/BP_BaseGamemode.SpawnCharacters` (`self.BaseGamemode`) (`|MakeArray` self :!type "/Game/Blueprints/BP_BasePlayerController Object Reference") false))

(event `self.ReceiveEndPlay`
  (params (EndPlayReason :type "EEndPlayReason Enum" :default "Destroyed"))
  (if (`self.IsLocalController`)
    (`Widget.RemoveFromParent` (`self.PlayerHUD`))
    (`Widget.RemoveFromParent` (`self.TransitionWidget`))
    (`Widget.RemoveFromParent` (`self.PauseWidget`))
    (`Widget.RemoveFromParent` (`self.GetGameHUD`))))

(event `SERVER_OnReady`
  (`/Game/Blueprints/BP_BaseGamemode.OnPlayerReady` (`/Game/BlueprintLibraries/Game.GetBaseGamemode`) self))

(event `CLIENT_SetupPlayer`
  (params (Map :type "/Game/Data/F_Map Structure") (Gamemode :type "/Game/Data/E_Gamemode Enum" :default "NewEnumerator0"))
  (`WidgetLayoutLibrary.RemoveAllWidgets`)
  (`self.CreateTransitionWidget`)
  (`self.CreatePauseMenu`)
  (`self.CreatePlayerHUD`)
  (`self.CreateGameHUD`)
  (set `self.Map` Map)
  (set `self.Gamemode` Gamemode)
  (set `self.Game Instance` (`/Game/BlueprintLibraries/Game.GetGameInstance`))
  (bind _returnvalue (`|SpawnActorFromClass` "/Game/Blueprints/BP_DeathCamera.BP_DeathCamera_C" (`self.GetTransform`) "AlwaysSpawn" "OverrideRootScale" null null))
  (set `self.DeathCamera` _returnvalue))

(event `CLIENT_StartPlayer`
  (`KismetSystemLibrary.Delay` 1.0)
  (`self.ShowPlayerHUD`)
  (`self.ShowGameHUD`)
  (`/Game/UserInterface/Menus/SubMenus/WBP_Transition.PlayTransition` (`self.GetTransitionWidget`) (delegate `EVENT`) "Reverse" 1.0)
  (`/Game/Blueprints/BP_GameInstance.Fade Persistent Sound` (`self.Game Instance`) 3.0)
  (`/Game/UserInterface/Menus/WBP_PauseMenu.UpdateGameData` (`self.GetPauseMenu`) (`self.Map`) (`self.Gamemode`)))

(event `EVENT`)

(event `CLIENT_OnPossess`
  (`/Game/Blueprints/BP_DeathCamera.DeactivateCamera` (`self.DeathCamera`))
  (`/Game/UserInterface/Gameplay/Components/WBP_RespawnUI.SetVisible` (`/Game/UserInterface/Gameplay/WBP_PlayerHUD.WBP_RespawnUI` (`self.GetPlayerHUD`)) false)
  (`KismetSystemLibrary.K2_ClearAndInvalidateTimerHandle` (`self.Timer_Respawn`))
  (`self.Set Spectating` false))

(event `CLIENT_OnUnpossess`
  (`KismetSystemLibrary.Delay` 3.0)
  (`self.Set Spectating` true)
  (bind _spectating_player (`self.OffsetPlayer` 0))
  (if (not _spectating_player)
    (`self.OffsetArenaCamera` 0)))

(event `SERVER_DealDamage`
  (params (`Target Actor` :type "Actor Object Reference") (Instigator :type "Actor Object Reference") (`Damage Data` :type "/Game/Data/F_DamageData Structure"))
  (message `/Game/BlueprintInterfaces/BI_Game.DamageActor` `Target Actor` Instigator `Damage Data`))

(event `SERVER_PickupItem`
  (params (Pickup :type "/Game/Blueprints/BP_BasePickup Object Reference"))
  (`/Game/Blueprints/BP_BasePickup.PickupItem (OnServer)` Pickup self (`self.PlayerCharacter`)))

(event `CLIENT_OnKill`
  (`GameplayStatics.PlaySound2D` "/Game/SFX/Gameplay/SC_MP_KILL.SC_MP_KILL" 1.0 1.0 0.0 null null))

(event `CLIENT_OnAssist`
  (`GameplayStatics.PlaySound2D` "/Game/SFX/Gameplay/SC_MP_ASSIST.SC_MP_ASSIST" 1.0 1.0 0.0 null null))

(event `CLIENT_OnDeath`
  (params (Killer :type "Actor Object Reference") (RespawnTime :type Integer))
  (bind _returnvalue (`GameplayStatics.GetPlayerCameraManager` 0))
  (`|ExecutionSequence`
    (:`then_0`
      (`self.StartRespawnTimer` RespawnTime))
    (:`then_1`
      (`KismetSystemLibrary.Delay` 0.2)
      (`/Game/Blueprints/BP_DeathCamera.ActivateCamera` (`self.DeathCamera`) Killer (`PlayerCameraManager.GetCameraLocation` _returnvalue) (`PlayerCameraManager.GetCameraRotation` _returnvalue)))))

(event `CLIENT_AddToGameFeed`
  (params (`Feed Data` :type "/Game/Data/F_FeedData Structure"))
  (`self.AddToGameFeed` `Feed Data`))

(event `CLIENT_ShowResults`
  (params (WinningTeam :type "/Game/Data/E_Team Enum" :default "NewEnumerator0"))
  (`self.ShowResults` WinningTeam)
  (`KismetSystemLibrary.Delay` 10.0)
  (`/Game/UserInterface/Menus/SubMenus/WBP_Transition.PlayTransition` (`self.GetTransitionWidget`) (delegate `EVENT_End`) "Forward" 3.0))

(event `EVENT_End`)

(event `CLIENT_StopRespawnTimer`
  (`self.StopRespawnTimer`))

(event `CLIENT_SpawnMoney`
  (params (Money :type Integer) (MoneyType :type "/Game/Data/E_MoneyType Enum" :default "NewEnumerator0") (Location :type "Vector Structure"))
  (`|SpawnActorFromClass` "/Game/Blueprints/BP_Money.BP_Money_C" (`KismetMathLibrary.MakeTransform` Location) "AlwaysSpawn" "OverrideRootScale" null Money MoneyType null))

(event `CLIENT_PlayGameMusic`
  (params (Index :type Integer))
  (`GameplayStatics.PlaySound2D` (select `int` Index :`0` "/Game/SFX/OST/SC_MP_POWERPLAY_01.SC_MP_POWERPLAY_01" :`1` "/Game/SFX/OST/SC_MP_POWERPLAY_02.SC_MP_POWERPLAY_02" :`2` "/Game/SFX/OST/SC_MP_POWERPLAY_03.SC_MP_POWERPLAY_03" :`3` "/Game/SFX/OST/SC_MP_POWERPLAY_04.SC_MP_POWERPLAY_04" :!type "SoundBase Object Reference") 1.0 1.0 0.0 null null))

(event `InputAction|Pause`
  (params (Key :type "Key Structure"))
  (:`Pressed`
    (if (not (`self.HasEnded`))
      (`self.ShowPauseMenu`))))

(event `InputAction|NextCamera`
  (params (Key :type "Key Structure"))
  (:`Pressed`
    (`self.OffsetArenaCamera` 1)))

(event `InputAction|PreviousCamera`
  (params (Key :type "Key Structure"))
  (:`Pressed`
    (`self.OffsetArenaCamera` -1)))

(event `InputAction|NextPlayer`
  (params (Key :type "Key Structure"))
  (:`Pressed`
    (`self.OffsetPlayer` 1)))

(event `InputAction|PreviousPlayer`
  (params (Key :type "Key Structure"))
  (:`Pressed`
    (`self.OffsetPlayer` -1)))

(event `InputAction|ShowScoreboard`
  (params (Key :type "Key Structure"))
  (:`Pressed`
    (if (not (`self.HasEnded`))
      (if (not (`self.IsScoreboardVisible`))
        (`self.ShowScoreboard`)
        (else
          (`self.HideScoreboard`))))))

(fn `AddTeammate`
  (params (Character :type "/Game/Blueprints/BP_BaseCharacter Object Reference"))
  (if (not (`KismetArrayLibrary.Array_Contains` (`self.Teammates`) Character))
    (`KismetArrayLibrary.Array_Add` (`self.Teammates`) (`local.Character`))))

(fn `AddToGameFeed`
  (params (`Feed Data` :type "/Game/Data/F_FeedData Structure")))

(fn `CreateGameHUD`)

(fn `CreatePauseMenu`
  (bind _returnvalue (`|CreateWidget` "/Game/UserInterface/Menus/WBP_PauseMenu.WBP_PauseMenu_C" (`GameplayStatics.GetPlayerController` 0)))
  (bind _output_get (set `self.PauseWidget` _returnvalue))
  (`UserWidget.AddToViewport` _output_get 999)
  (`self.HidePauseMenu`))

(fn `CreatePlayerHUD`
  (bind _returnvalue (`|CreateWidget` "/Game/UserInterface/Gameplay/WBP_PlayerHUD.WBP_PlayerHUD_C" (`GameplayStatics.GetPlayerController` 0)))
  (bind _output_get (set `self.PlayerHUD` _returnvalue))
  (`UserWidget.AddToViewport` _output_get 0)
  (`self.HidePlayerHUD`))

(fn `CreateTransitionWidget`
  (bind _returnvalue (`|CreateWidget` "/Game/UserInterface/Menus/SubMenus/WBP_Transition.WBP_Transition_C" (`GameplayStatics.GetPlayerController` 0)))
  (bind _output_get (set `self.TransitionWidget` _returnvalue))
  (`UserWidget.AddToViewport` _output_get 499)
  (`/Game/UserInterface/Menus/SubMenus/WBP_Transition.FillScreen` (`self.GetTransitionWidget`))
  (`KismetSystemLibrary.PrintString` "Transition Widget created"))

(fn `GetAssists`
  (returns (Assists :type Integer))
  (bind _assists (message `/Game/BlueprintInterfaces/BI_Game.GetAssists` (`self.PlayerState`)))
  (return _assists))

(fn `GetDeaths`
  (returns (Deaths :type Integer))
  (bind _deaths (message `/Game/BlueprintInterfaces/BI_Game.GetDeaths` (`self.PlayerState`)))
  (return _deaths))

(fn `GetEntityName`
  (returns (Name :type Text))
  (return (`KismetTextLibrary.Conv_StringToText` (`PlayerState.GetPlayerName` (`self.PlayerState`)))))

(fn `GetFocusLocation`
  (returns (Location :type "Vector Structure"))
  (return (0.0 0.0 0.0)))

(fn `GetGameHUD`
  (returns (Widget :type "UserWidget Object Reference"))
  (return null))

(fn `GetGamemode`
  (returns (Gamemode :type "/Game/Data/E_Gamemode Enum"))
  (return (`self.Gamemode`)))

(fn `GetKills`
  (returns (Kills :type Integer))
  (bind _kills (message `/Game/BlueprintInterfaces/BI_Game.GetKills` (`self.PlayerState`)))
  (return _kills))

(fn `GetMoneyLocation`
  (returns (Location :type "Vector Structure"))
  (return (0.0 0.0 0.0)))

(fn `GetPauseMenu`
  (returns (`Return Value` :type "/Game/UserInterface/Menus/WBP_PauseMenu Object Reference"))
  (return (`self.PauseWidget`)))

(fn `GetPlayerHUD`
  (returns (PlayerHUD :type "/Game/UserInterface/Gameplay/WBP_PlayerHUD Object Reference"))
  (return (`self.PlayerHUD`)))

(fn `GetScore`
  (returns (Score :type Integer))
  (bind _score (message `/Game/BlueprintInterfaces/BI_Game.GetScore` (`self.PlayerState`)))
  (return _score))

(fn `GetSightLocation`
  (returns (Location :type "Vector Structure"))
  (return (0.0 0.0 0.0)))

(fn `GetTeam`
  (returns (Team :type "/Game/Data/E_Team Enum"))
  (return (`self.PlayerTeam`)))

(fn `GetTransitionWidget`
  (returns (TransitionWidget :type "/Game/UserInterface/Menus/SubMenus/WBP_Transition Object Reference"))
  (return (`self.TransitionWidget`)))

(fn `HideGameHUD`
  (set `self.IsScoreboardVisible` false))

(fn `HidePauseMenu`
  (`self.ShowPlayerHUD`)
  (`self.ShowGameHUD`)
  (`Widget.SetVisibility` (`self.GetPauseMenu`) "Hidden")
  (`WidgetBlueprintLibrary.SetInputMode_GameOnly` (`GameplayStatics.GetPlayerController` 0))
  (set `self.bShowMouseCursor` false))

(fn `HidePlayerHUD`
  (`Widget.SetVisibility` (`self.PlayerHUD`) "Collapsed"))

(fn `HideScoreboard`
  (set `self.IsScoreboardVisible` false))

(fn `IsCritical`
  (params (`Hit Bone` :type Name))
  (returns (IsCritical :type Boolean))
  (return false))

(fn `OffsetArenaCamera`
  (params (Offset :type Integer))
  (bind _returnvalue (- (`KismetArrayLibrary.Array_Length` (`self.ArenaCameras`)) 1))
  (if (`self.IsSpectating`)
    (if (not (== Offset 0))
      (bind _output_get (set `self.CameraIndex` (+ Offset (`self.CameraIndex`))))
      (if (> _output_get _returnvalue)
        (set `self.CameraIndex` 0)
        (elif (< (`self.CameraIndex`) 0)
          (set `self.CameraIndex` _returnvalue))))
    (`/Game/Blueprints/BP_ArenaCamera.SpectateCamera` (`|GetArrayItem` (`self.ArenaCameras`) (`self.CameraIndex`)))))

(fn `OffsetPlayer`
  (params (Offset :type Integer))
  (returns (`Spectating Player` :type Boolean))
  (bind _returnvalue (- (`KismetArrayLibrary.Array_Length` (`self.Teammates`)) 1))
  (if (`KismetArrayLibrary.Array_IsEmpty` (`self.Teammates`))
    (return false)
    (elif (`self.IsSpectating`)
      (if (not (== Offset 0))
        (bind _output_get (set `self.PlayerIndex` (+ Offset (`self.PlayerIndex`))))
        (if (< _output_get 0)
          (set `self.PlayerIndex` _returnvalue)
          (elif (> _output_get _returnvalue)
            (set `self.PlayerIndex` 0))))
      (`self.SpectatePlayer` (`|GetArrayItem` (`self.Teammates`) (`self.PlayerIndex`)))
      (return true))))

(fn `OnDeath (OnServer)`
  (params (Object :type "Object Object Reference"))
  (bind _basegamemode (`self.BaseGamemode`))
  (bind _basegamemode_2 (`self.BaseGamemode`))
  (bind _returnvalue (`/Game/Blueprints/BP_BaseGamemode.UseRespawnWaves` (`self.BaseGamemode`)))
  (bind _match_respawninterval (`/Game/Blueprints/BP_BaseGamemode.GetRespawnInterval` _basegamemode_2))
  (bind _returnvalue_2 (mod (`/Game/Blueprints/BP_BaseGamemode.GetTime` _basegamemode_2) _match_respawninterval))
  (bind _returnvalue_3 (<= _returnvalue_2 4))
  (`/Game/Blueprints/BP_BasePlayerState.OffsetDeaths` (`self.BasePlayerState`) 1)
  (`self.CLIENT_OnDeath` (`/Game/Blueprints/BP_BasePlayerController.PlayerCharacter` (cast `/Game/Blueprints/BP_BasePlayerController` Object :!pure true)) (- (`KismetMathLibrary.SelectInt` (`KismetMathLibrary.SelectInt` (+ _match_respawninterval _returnvalue_2) _returnvalue_2 _returnvalue_3) _match_respawninterval _returnvalue) 1))
  (if _returnvalue
    (if _returnvalue_3
      (`/Game/Blueprints/BP_BaseGamemode.AddPlayerToDeadQueue` _basegamemode self)
      (else
        (`/Game/Blueprints/BP_BaseGamemode.AddPlayerToDeadList` _basegamemode self)))
    (else
      (`self.StartServer_RespawnTimer` (`/Game/Blueprints/BP_BaseGamemode.GetRespawnInterval` (`self.BaseGamemode`))))))

(fn `OnGameResult`
  (params (Result :type "/Game/Data/E_GameResult Enum" :default "NewEnumerator0"))
  (`AudioComponent.FadeOut` (`self.AUDIO_GameMusic`) 3.0 0.0 "Linear")
  (switch `/Game/Data/E_GameResult` Result
    (:`NewEnumerator1`
      (`GameplayStatics.PlaySound2D` "/Game/SFX/OST/SC_MP_WIN.SC_MP_WIN" 1.0 1.0 0.0 null null))
    (:`NewEnumerator2`
      (`GameplayStatics.PlaySound2D` "/Game/SFX/OST/SC_MP_LOSS.SC_MP_LOSS" 1.0 1.0 0.0 null null :!label _label))
    (:`NewEnumerator3`
      (goto _label))))

(fn `OnRep_PlayerStates`
  (if (`self.IsLocalController`)
    (`self.OnReady`)
    (if (not (`self.HasEnded`))
      (`self.Update Scoreboard`))))

(fn `RemoveTeammate`
  (params (Character :type "/Game/Blueprints/BP_BaseCharacter Object Reference"))
  (bind _spectatingplayer (`self.SpectatingPlayer`))
  (bind _returnvalue (`KismetArrayLibrary.Array_RemoveItem` (`self.Teammates`) Character))
  (if _returnvalue
    (if (and (`self.IsSpectating`) (`KismetSystemLibrary.IsValid` _spectatingplayer))
      (if (== Character _spectatingplayer)
        (bind _spectating_player (`self.OffsetPlayer` 0))
        (if (not _spectating_player)
          (`self.OffsetArenaCamera` 0))))))

(fn `Set Spectating`
  (params (NewValue :type Boolean))
  (bind _output_get (set `self.IsSpectating` NewValue))
  (if (not _output_get)
    (`/Engine/EditorBlueprintResources/StandardMacros.IsValid` (`self.SpectatingPlayer`)
      (:`Is Valid`
        (`/Game/Blueprints/BP_BaseCharacter.SetIsSpectating` (`self.SpectatingPlayer`) false)))))

(fn `SetIsDead`
  (params (NewValue :type Boolean))
  (`/Game/Blueprints/BP_BasePlayerState.SetIsDead` (`self.BasePlayerState`) NewValue))

(fn `SetNewWeapon`
  (params (MagSize :type Integer))
  (`/Game/UserInterface/Gameplay/Components/WBP_EquipmentDisplay.SetNewWeapon` (`/Game/UserInterface/Gameplay/WBP_PlayerHUD.WBP_EquipmentDisplay` (`self.GetPlayerHUD`)) MagSize))

(fn `SetPlayerStates`
  (params (PlayerStates :type "Array of /Game/Blueprints/BP_BasePlayerState Object Reference"))
  (set `self.PlayerStates` PlayerStates))

(fn `SetTeam`
  (params (NewTeam :type "/Game/Data/E_Team Enum" :default "NewEnumerator0"))
  (returns (Team :type "/Game/Data/E_Team Enum"))
  (bind _output_get (set `self.PlayerTeam` NewTeam))
  (bind _asbp_base_player_state (cast `/Game/Blueprints/BP_BasePlayerState` (`self.PlayerState`)))
  (`/Game/Blueprints/Lobby/BP_LobbyPlayerState.SERVER_SetTeam` _asbp_base_player_state _output_get)
  (return _output_get))

(fn `ShowGameHUD`)

(fn `ShowPauseMenu`
  (`self.HidePlayerHUD`)
  (`self.HideGameHUD`)
  (`Widget.SetVisibility` (`self.GetPauseMenu`) "SelfHitTestInvisible")
  (`WidgetBlueprintLibrary.SetInputMode_UIOnlyEx` self (`self.GetPauseMenu`))
  (set `self.bShowMouseCursor` true)
  (`/Game/UserInterface/Menus/WBP_PauseMenu.SetupPauseMenu` (`self.GetPauseMenu`)))

(fn `ShowPlayerHUD`
  (`Widget.SetVisibility` (`self.PlayerHUD`) "HitTestInvisible"))

(fn `ShowResults`
  (params (WinningTeam :type "/Game/Data/E_Team Enum" :default "NewEnumerator0"))
  (`self.HidePauseMenu`)
  (`self.HidePlayerHUD`)
  (`self.ShowScoreboard`)
  (set `self.HasEnded` true))

(fn `ShowScoreboard`
  (set `self.IsScoreboardVisible` true))

(fn `SpectatePlayer`
  (params (Player :type "/Game/Blueprints/BP_BaseCharacter Object Reference"))
  (bind _spectatingplayer (`self.SpectatingPlayer`))
  (`|ExecutionSequence`
    (:`then_0`
      (`/Engine/EditorBlueprintResources/StandardMacros.IsValid` _spectatingplayer
        (:`Is Valid`
          (`/Game/Blueprints/BP_BaseCharacter.SetIsSpectating` _spectatingplayer false))))
    (:`then_1`
      (`self.SetViewTargetWithBlend` Player)
      (bind _output_get (set `self.SpectatingPlayer` Player))
      (`/Game/Blueprints/BP_BaseCharacter.SetIsSpectating` _output_get true))))

(fn `StopRespawnTimer`
  (`KismetSystemLibrary.K2_ClearAndInvalidateTimerHandle` (`self.Timer_Respawn`)))

(fn `Update Scoreboard`)

(fn `UpdateCurrentWeaponState`
  (params (State :type "/Game/Data/F_WeaponState Structure"))
  (`/Game/UserInterface/Gameplay/Components/WBP_EquipmentDisplay.UpdateWeaponState` (`/Game/UserInterface/Gameplay/WBP_PlayerHUD.WBP_EquipmentDisplay` (`self.GetPlayerHUD`)) State))

(fn `UserConstructionScript`)