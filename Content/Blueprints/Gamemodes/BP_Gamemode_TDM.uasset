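; Team Deathmatch game mode Blueprint that applies match options for time and respawn time.
; HandleGameOptions switches on the option type, looks up the selected choice in the matching options map, and passes the value to SetTime or SetRespawnInterval.
; BeginPlay and the construction script only call their parent versions.
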(event `self.ReceiveBeginPlay`
  (`parent.ReceiveBeginPlay`))

(fn `HandleGameOptions`
  (params (Option :type String) (SelectedOption :type Integer))
  (switch `string` Option
    (:`time`
      (`self.SetTime` (`BlueprintMapLibrary.Map_Find` (`self.Options_Time`) SelectedOption)))
    (:`respawn time`
      (`self.SetRespawnInterval` (`BlueprintMapLibrary.Map_Find` (`self.Options_Respawn`) SelectedOption)))))

(fn `UserConstructionScript`
  (`parent.UserConstructionScript`))