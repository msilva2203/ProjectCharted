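; BP_Gamemode_FFA is the free-for-all game mode, handling match setup, options and winner selection.
; On match start it sets the goal on BP_GameState_FFA, zeroes eight team scores and forwards time updates to it.
; Option handling maps selections to game time, respawn interval, respawn waves and objective goal.
; FindWinningTeam scans players' team scores for the highest, using the first enumerator when a score is zero.
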(event `self.ReceiveBeginPlay`
  (`parent.ReceiveBeginPlay`))

(event `PrepareGamemode`
  (bind _asbp_game_state_ffa (cast `/Game/Blueprints/Gamestates/BP_GameState_FFA` (`GameplayStatics.GetGameState`)))
  (bind _output_get (set `self.GameState_FFA` _asbp_game_state_ffa))
  (`/Game/Blueprints/Gamestates/BP_GameState_FFA.SetGoal` _output_get (`self.Goal`))
  (for _array_element (`|MakeArray` "NewEnumerator1" "NewEnumerator2" "NewEnumerator3" "NewEnumerator4" "NewEnumerator5" "NewEnumerator6" "NewEnumerator7" "NewEnumerator8" :!type "/Game/Data/E_Team Enum")
    (`/Game/Blueprints/Gamestates/BP_GameState_FFA.SetTeamScore` (`self.GameState_FFA`) _array_element 0))
  (add `self.OnTimeUpdate` (delegate `EVENT_OnTimeUpdated`)))

(event `EVENT_OnTimeUpdated` :!signature `self.OnTimeUpdate`
  (params (Time :type Integer))
  (`/Game/Blueprints/Gamestates/BP_GameState_FFA.SetTime` (`self.GameState_FFA`) Time))

(fn `FindWinningTeam`
  (returns (Team :type "/Game/Data/E_Team Enum"))
  (locals (TEMP_Biggest :type Integer) (TEMP_Current :type Integer :default 0) (TEMP_Team :type "/Game/Data/E_Team Enum"))
  (for _array_element (`self.Players`)
    (bind _team (`/Game/BlueprintInterfaces/BI_Game.GetTeam` _array_element))
    (bind _output_get (set `local.TEMP_Current` (`/Game/Blueprints/Gamestates/BP_GameState_FFA.GetTeamScore` (`self.GameState_FFA`) _team)))
    (if (>= _output_get (`local.TEMP_Biggest`))
      (if (== (`local.TEMP_Current`) 0)
        (set `local.TEMP_Team` "NewEnumerator0")
        (else
          (set `local.TEMP_Biggest` (`local.TEMP_Current`))
          (set `local.TEMP_Team` _team)))))
  (return (`local.TEMP_Team`)))

(fn `HandleGameOptions`
  (params (Option :type String) (SelectedOption :type Integer))
  (switch `string` Option
    (:`game time`
      (`self.SetTime` (`BlueprintMapLibrary.Map_Find` (`self.Options_Time`) SelectedOption)))
    (:`respawn time`
      (`self.SetRespawnInterval` (`BlueprintMapLibrary.Map_Find` (`self.Options_RespawnTime`) SelectedOption)))
    (:`objective goal`
      (`self.SetGoal` (`BlueprintMapLibrary.Map_Find` (`self.Options_Goal`) SelectedOption)))
    (:`use respawn waves`
      (`self.SetUseRespawnWaves` (`KismetMathLibrary.Conv_IntToBool` SelectedOption)))))

(fn `SetGoal`
  (params (Goal :type Integer))
  (set `self.Goal` Goal))

(fn `StartMatch`
  (`parent.StartMatch`)
  (`self.PrepareGamemode`))

(fn `UserConstructionScript`
  (`parent.UserConstructionScript`))