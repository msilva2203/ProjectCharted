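; Player state Blueprint for the TTDM game mode that keeps the player's entry display in sync with their stats.
; It stores a PlayerEntry reference through SetPlayerEntry.
; Handlers for kills, deaths and assists changes write each value to its own stat slot on that entry, and the dead-state handler forwards the Dead flag to it.
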(fn `OnAssistsSet`
  (bind _assists (`/Game/BlueprintInterfaces/BI_Game.GetAssists`))
  (`/Game/UserInterface/Gameplay/Components/WBP_PlayerScoreboardEntry.SetStat` (`self.Player Entry`) 2 _assists))

(fn `OnDeathsSet`
  (bind _deaths (`/Game/BlueprintInterfaces/BI_Game.GetDeaths`))
  (`/Game/UserInterface/Gameplay/Components/WBP_PlayerScoreboardEntry.SetStat` (`self.Player Entry`) 1 _deaths))

(fn `OnIsDeadSet`
  (`/Game/UserInterface/Gameplay/Components/WBP_PlayerScoreboardEntry.SetIsDead` (`self.Player Entry`) (`self.Dead`)))

(fn `OnKillsSet`
  (bind _kills (`/Game/BlueprintInterfaces/BI_Game.GetKills`))
  (`/Game/UserInterface/Gameplay/Components/WBP_PlayerScoreboardEntry.SetStat` (`self.Player Entry`) 0 _kills))

(fn `SetPlayerEntry`
  (params (PlayerEntry :type "/Game/UserInterface/Gameplay/Components/WBP_PlayerScoreboardEntry Object Reference"))
  (set `self.Player Entry` PlayerEntry))

(fn `UserConstructionScript`
  (`parent.UserConstructionScript`))