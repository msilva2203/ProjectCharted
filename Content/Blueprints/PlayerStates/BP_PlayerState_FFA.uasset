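; BP_PlayerState_FFA is the player state for free-for-all mode, linking a player's kill and death counts to a scoreboard entry.
; SetScoreboardEntry stores the entry reference.
; OnKillsSet and OnDeathsSet read the current kills and deaths and write them into the entry's first and second stat slots.
; BeginPlay and Tick are unused, so updates come only through those setter callbacks.
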(fn `OnDeathsSet`
  (bind _deaths (`/Game/BlueprintInterfaces/BI_Game.GetDeaths`))
  (`/Game/UserInterface/Gameplay/Components/WBP_PlayerScoreboardEntry.SetStat` (`self.Scoreboard Entry`) 1 _deaths))

(fn `OnKillsSet`
  (bind _kills (`/Game/BlueprintInterfaces/BI_Game.GetKills`))
  (`/Game/UserInterface/Gameplay/Components/WBP_PlayerScoreboardEntry.SetStat` (`self.Scoreboard Entry`) 0 _kills))

(fn `SetScoreboardEntry`
  (params (ScoreboardEntry :type "/Game/UserInterface/Gameplay/Components/WBP_PlayerScoreboardEntry Object Reference"))
  (set `self.Scoreboard Entry` ScoreboardEntry))

(fn `UserConstructionScript`
  (`parent.UserConstructionScript`))