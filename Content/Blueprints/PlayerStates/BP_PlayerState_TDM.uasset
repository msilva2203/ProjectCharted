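; Team Deathmatch player state that mirrors a player's kills, deaths, assists and dead status into their linked scoreboard entry.
; Assigning an entry pushes all three stats at once, and each stat setter callback updates its own column afterward.
; IsWorse ranks players by most kills, then fewest deaths, then most assists.
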(fn `Is Worse`
  (params (OtherPlayer :type "/Game/Blueprints/PlayerStates/BP_PlayerState_TDM Object Reference"))
  (returns (ReturnValue :type Boolean))
  (bind _kills (`/Game/BlueprintInterfaces/BI_Game.GetKills` OtherPlayer))
  (bind _kills_2 (`/Game/BlueprintInterfaces/BI_Game.GetKills`))
  (if (> _kills _kills_2)
    (return true)
    (elif (== _kills _kills_2)
      (bind _deaths (`/Game/BlueprintInterfaces/BI_Game.GetDeaths` OtherPlayer))
      (bind _deaths_2 (`/Game/BlueprintInterfaces/BI_Game.GetDeaths`))
      (if (< _deaths _deaths_2)
        (return true)
        (elif (== _deaths _deaths_2)
          (bind _assists (`/Game/BlueprintInterfaces/BI_Game.GetAssists` OtherPlayer))
          (bind _assists_2 (`/Game/BlueprintInterfaces/BI_Game.GetAssists`))
          (return (> _assists _assists_2))
          (else
            (return false))))
      (else
        (return false)))))

(fn `OnAssistsSet`
  (bind _assists (`/Game/BlueprintInterfaces/BI_Game.GetAssists`))
  (`/Game/UserInterface/Gameplay/Components/WBP_PlayerScoreboardEntry.SetStat` (`self.ScoreboardEntry`) 2 _assists))

(fn `OnDeathsSet`
  (bind _deaths (`/Game/BlueprintInterfaces/BI_Game.GetDeaths`))
  (`/Game/UserInterface/Gameplay/Components/WBP_PlayerScoreboardEntry.SetStat` (`self.ScoreboardEntry`) 1 _deaths))

(fn `OnIsDeadSet`
  (`/Game/UserInterface/Gameplay/Components/WBP_PlayerScoreboardEntry.SetIsDead` (`self.ScoreboardEntry`) (`self.Dead`)))

(fn `OnKillsSet`
  (bind _kills (`/Game/BlueprintInterfaces/BI_Game.GetKills`))
  (`/Game/UserInterface/Gameplay/Components/WBP_PlayerScoreboardEntry.SetStat` (`self.ScoreboardEntry`) 0 _kills))

(fn `SetScoreboardEntry`
  (params (ScoreboardEntry :type "/Game/UserInterface/Gameplay/Components/WBP_PlayerScoreboardEntry Object Reference"))
  (set `self.ScoreboardEntry` ScoreboardEntry)
  (`self.Update Scoreboard Stats`))

(fn `Update Scoreboard Stats`
  (`|ExecutionSequence`
    (:`then_0`
      (bind _kills (`/Game/BlueprintInterfaces/BI_Game.GetKills`))
      (`/Game/UserInterface/Gameplay/Components/WBP_PlayerScoreboardEntry.SetStat` (`self.ScoreboardEntry`) 0 _kills))
    (:`then_1`
      (bind _deaths (`/Game/BlueprintInterfaces/BI_Game.GetDeaths`))
      (`/Game/UserInterface/Gameplay/Components/WBP_PlayerScoreboardEntry.SetStat` (`self.ScoreboardEntry`) 1 _deaths))
    (:`then_2`
      (bind _assists (`/Game/BlueprintInterfaces/BI_Game.GetAssists`))
      (`/Game/UserInterface/Gameplay/Components/WBP_PlayerScoreboardEntry.SetStat` (`self.ScoreboardEntry`) 2 _assists))))

(fn `UserConstructionScript`
  (`parent.UserConstructionScript`))