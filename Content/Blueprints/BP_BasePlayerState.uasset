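; Base player state that tracks a player's kills, assists, deaths and score for a match.
; Each stat has a server-named event that adds an offset, then passes the new total to a NETALL-named event that sets it, apparently as a multicast to all machines.
; Simple getter functions expose each value to other Blueprints.
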(event `SERVER_OffsetKills`
  (params (Offset :type Integer))
  (bind _output_get (set `self.Kills` (+ Offset (`self.Kills`))))
  (`self.NETALL_SetKills` _output_get))

(event `NETALL_SetKills`
  (params (NewValue :type Integer))
  (set `self.Kills` NewValue))

(event `SERVER_OffsetAssists`
  (params (Offset :type Integer))
  (bind _output_get (set `self.Assists` (+ Offset (`self.Assists`))))
  (`self.NETALL_SetAssists` _output_get))

(event `NETALL_SetAssists`
  (params (NewValue :type Integer))
  (set `self.Assists` NewValue))

(event `SERVER_OffsetDeaths`
  (params (Offset :type Integer))
  (bind _output_get (set `self.Deaths` (+ Offset (`self.Deaths`))))
  (`self.NETALL_SetDeaths` _output_get))

(event `NETALL_SetDeaths`
  (params (NewValue :type Integer))
  (set `self.Deaths` NewValue))

(event `SERVER_OffsetScore`
  (params (Offset :type Integer))
  (bind _output_get (set `self.PlayerScore` (+ Offset (`self.PlayerScore`))))
  (`self.NETALL_SetScore` _output_get))

(event `NETALL_SetScore`
  (params (NewValue :type Integer))
  (set `self.PlayerScore` NewValue))

(fn `GetAssists`
  (returns (Assists :type Integer))
  (return (`self.Assists`)))

(fn `GetDeaths`
  (returns (Deaths :type Integer))
  (return (`self.Deaths`)))

(fn `GetKills`
  (returns (Kills :type Integer))
  (return (`self.Kills`)))

(fn `GetScore`
  (returns (Score :type Integer))
  (return (`self.PlayerScore`)))

(fn `UserConstructionScript`)